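; Herb pickup item for the inventory system that restores the player's stamina when used.
; On Interact it adds one of its item to the interactor's Bp_InventorySystem component and destroys itself if that succeeds.
; UseItem runs the parent logic, then adds a fixed amount of Stamina to player 0's TopDownCharacter, with no clamp here, and returns the parent's result.
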(event EventBeginPlay)

(event Collision|EventActorBeginOverlap
  (params (OtherActor :type Actor%20Object%20Reference)))

(event EventTick
  (params (DeltaSeconds :type Float%20%28single-precision%29)))

(event EventInteract
  (params (Interactor :type Actor%20Object%20Reference))
  (bind _succes_ (Default|AddtoInventory (Actor|GetComponentbyClass Interactor "/Game/Blueprints/InventorySystem/Bp_InventorySystem.Bp_InventorySystem_C") (Utilities|Struct|MakeE_SlotStructure (Variables|Default|GetItemStructure) 1)))
  (if _succes_
    (Actor|DestroyActor)))

(fn ConstructionScript
  (|CallParentFunction))

(fn UseItem
  (bind _success_ (|CallParentFunction))
  (bind _astop_down_character (Utilities|Casting|CastToTopDownCharacter (Game|GetPlayerCharacter 0)))
  (Variables|/Game/Blueprints/TopDownCharacter.TopDownCharacter_C|SetStamina _astop_down_character (+ (Variables|/Game/Blueprints/TopDownCharacter.TopDownCharacter_C|GetStamina _astop_down_character) 3e+01))
  (return _success_))