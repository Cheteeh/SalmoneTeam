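; Inventory component that stores items as a map of item name to quantity, with functions to add, remove and transfer them.
; Adding stacks onto an existing entry or creates a new one.
; Removal succeeds only when enough quantity is held, deletes the entry when it reaches zero, and returns whether it worked.
; Swap is a one-way transfer that adds to the target inventory only if removal from this one succeeds.
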(fn AddtoInventory
  (params (ItemName :type Name) (Quantity :type Integer))
  (bind _inventorycontent (Variables|Default|GetInventoryContent))
  (bind (_value _returnvalue) (Utilities|Map|Find _inventorycontent ItemName))
  ;[1 1 1] Busca si hay un objeto de ese tipo en el inventario y setea la cantidad
  (Utilities|Map|Add _inventorycontent ItemName (Math|Integer|SelectInt (+ Quantity _value) Quantity _returnvalue)))

(fn RemovefromInventory
  (params (ItemName :type Name) (Quantity :type Integer))
  (bind _inventorycontent (Variables|Default|GetInventoryContent))
  (bind _value (Utilities|Map|Find _inventorycontent ItemName))
  (bind _returnvalue (- _value Quantity))
  ;[1 1 1] Comprueba si hay suficientes en el inventario
  (if (<= Quantity _value)
    ;[1 1 1] Si hay suficientes objetos en el inventario elimina los necesarios o todos si es el caso
    (if (== _returnvalue 0)
      (Utilities|Map|Remove (Variables|Default|GetInventoryContent) ItemName)
      (return true)
      (else
        (Utilities|Map|Add (Variables|Default|GetInventoryContent) ItemName _returnvalue)
        (return true)))
    (else
      (return false) ; Devuelve si no hay objetos en el inventario
    )))

(fn SwapwithInventory
  (params (TargetInventory :type Inventory%20Component%20Object%20Reference) (ItemName :type Name) (Quantity :type Integer))
  (bind _success_ (CallFunction|RemovefromInventory ItemName Quantity))
  (if _success_
    (CallFunction|AddtoInventory TargetInventory ItemName Quantity)
    (return 0)))