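; InventoryComponent is an inventory component that tracks item quantities in a map keyed by item name.
; AddToInventory adds the quantity to any existing count or creates a new entry.
; RemoveFromInventory returns false when the stored count is too low; otherwise it subtracts the amount, deletes entries that reach zero, and returns true.
; SwapWithInventory is an empty stub.
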(fn AddtoInventory
  (params (ItemName :type Name) (Quantity :type Integer))
  (bind _inventorycontent (Variables|Default|GetInventoryContent))
  (bind (_value _returnvalue) (Utilities|Map|Find _inventorycontent ItemName))
  (Utilities|Map|Add _inventorycontent ItemName (Math|Integer|SelectInt (+ Quantity _value) Quantity _returnvalue)))

(fn RemovefromInventory
  (params (ItemName :type Name) (Quantity :type Integer))
  (bind _inventorycontent (Variables|Default|GetInventoryContent))
  (bind _value (Utilities|Map|Find _inventorycontent ItemName))
  (bind _returnvalue (- _value Quantity))
  (if (<= Quantity _value)
    (if (== _returnvalue 0)
      (Utilities|Map|Remove (Variables|Default|GetInventoryContent) ItemName)
      (return true)
      (else
        (Utilities|Map|Add (Variables|Default|GetInventoryContent) ItemName _returnvalue)
        (return true)))
    (else
      (return false))))

(fn SwapwithInventory)