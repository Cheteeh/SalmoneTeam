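; Bp_MasterUnit is a unit for a tile-based team game, with health, damage and movement between tiles.
; InteractWithTile attacks an occupant of another team and resets position, or sets a move target at an empty tile's "Centro" socket.
; Tick interpolates toward that target with a fixed, frame-rate-dependent step, then disables itself.
; ApplyDamage destroys the unit at zero Hp; ResetPosition returns the mesh to coordinates saved from overlapping box components.
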(event Custom|GetCurrentSocketLocation
  (bind _staticmesh (Variables|Default|GetStaticMesh))
  (bind _outoverlappingcomponents (Class|PrimitiveComponent|GetOverlappingComponents _staticmesh))
  (for _index (range 0 (Utilities|Array|Length _outoverlappingcomponents))
    (bind _asbox_collision (Utilities|Casting|CastToBoxComponent (Utilities|Array|Get(acopy) _outoverlappingcomponents _index)))
    (Variables|Default|SetLastTileCoords (Transformation|GetWorldLocation _asbox_collision))))

(event EventTick
  (params (DeltaSeconds :type Float%20%28single-precision%29))
  (if (Variables|Default|GetMove?)
    (if (Math|Vector|Equal(Vector) (Transformation|GetActorLocation) (Variables|Default|GetMoveTo) 0.0001)
      (Variables|Default|SetMove? false)
      (Actor|Tick|SetActorTickEnabled false)
      (else
        (Transformation|SetActorLocation (Math|Interpolation|VInterpTo (Transformation|GetActorLocation) (Variables|Default|GetMoveTo) 1.0 0.1) false false)))))

(fn ConstructionScript)

(fn ApplyDamage
  (params (Damage :type Integer))
  (bind _output_get (Variables|Default|SetHp (- (Variables|Default|GetHp) Damage)))
  (Development|PrintString (Utilities|String|ToString(Integer) _output_get) true true "(R=0.677732,G=1.000000,B=0.000000,A=1.000000)")
  (if (<= _output_get 0)
    (Development|PrintString "Muerto")
    (Actor|DestroyActor)
    (else
      (Development|PrintString "Daño Aplicado"))))

(fn InteractwithTile
  (params (TargetTile :type Bp%20Terrain%20Object%20Reference) (NoTile :type Boolean))
  (if NoTile
    (CallFunction|ResetPosition)
    (else
      ;[1 1 1] Tile local Var
      (bind _output_get (LocalVariables|SetTile TargetTile))
      ;[1 1 1] Occupied?
      (if (Variables|/Game/Blueprint/Grid/Bp_Terrain.Bp_Terrain_C|GetEstaOcupada? _output_get)
        ;[1 1 1] Ocuppied, attack and reset move
        (bind _asbp_master_unit (Utilities|Casting|CastToBp_MasterUnit (Variables|/Game/Blueprint/Grid/Bp_Terrain.Bp_Terrain_C|GetQuienMeocupa (LocalVariables|GetTile))))
        (if (!= (Variables|Bp_MasterUnit_C|GetTeam _asbp_master_unit) (Variables|Default|GetTeam))
          (CallFunction|ApplyDamage _asbp_master_unit (Variables|Default|GetDamage)))
        (CallFunction|ResetPosition)
        (else
          ;[1 1 1] Not occupied, move
          (Variables|Default|SetMoveTo (Transformation|GetSocketLocation (Variables|/Script/Engine.Actor|GetRootComponent (LocalVariables|GetTile)) "Centro"))
          (Variables|Default|SetMove? true)
          (Actor|Tick|SetActorTickEnabled true))))))

(fn ResetPosition
  (Transformation|SetWorldLocation (Variables|Default|GetStaticMesh) (Variables|Default|GetLastTileCoords) false false))