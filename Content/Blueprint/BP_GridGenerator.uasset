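; BP_GridGenerator builds a staggered tile board, populates it with two teams of units and drives timed turns.
; The construction script lays out offset preview meshes and splits their indices into per-team spawn tables.
; BeginPlay swaps each mesh for a Bp_Terrain actor, then spawns Bp_MasterUnits on shuffled positions with team materials.
; Tick calls NextTurn on every terrain tile whenever the TimeToTurn interval elapses.
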(event EventBeginPlay
  (Utilities|FlowControl|Sequence
    (:then_0
      ;[1 1 1] Create Bp_Terrain Actors and Destroy Mesh From Autogenerator
      (for _array_element (Variables|Grid|GetTiles)
        (bind _returnvalue (Game|SpawnActorfromClass "/Game/Blueprint/Bp_Terrain.Bp_Terrain_C" (Math|Transform|MakeTransform (Transformation|GetWorldLocation _array_element) "0, 0, 0" "1,1,1") "Undefined" 0 0))
        (Utilities|Array|Add (Variables|Grid|GetActor_Tiles) _returnvalue)
        (Components|DestroyComponent _array_element)))
    (:then_1
      ;[1 1 1] Player Tokens Spawn
      (Utilities|Array|Shuffle (Variables|Default|Getn_Units_P1_Positions))
      (for _index (range 0 (- (Variables|Default|Getn_Units_P1) 1))
        (bind _asbp_terrain (Utilities|Casting|CastToBp_Terrain (Utilities|Array|Get(acopy) (Variables|Grid|GetActor_Tiles) (Utilities|Array|Get(acopy) (Variables|Default|Getn_Units_P1_Positions) _index))))
        (bind _returnvalue_2 (Game|SpawnActorfromClass "/Game/Blueprint/Bp_MasterUnit.Bp_MasterUnit_C" (Math|Transform|MakeTransform (Transformation|GetSocketLocation (Variables|/Game/Blueprint/Bp_Terrain.Bp_Terrain_C|GetStaticMesh _asbp_terrain) "Centro") "0, 0, 0" "1,1,1") "Undefined" 0 0))
        (bind _asbp_master_unit (Utilities|Casting|CastToBp_MasterUnit _returnvalue_2))
        (Variables|/Game/Blueprint/Bp_MasterUnit.Bp_MasterUnit_C|SetTeam _asbp_master_unit 1)
        (Rendering|Material|SetMaterial (Variables|/Game/Blueprint/Bp_MasterUnit.Bp_MasterUnit_C|GetStaticMesh _asbp_master_unit) 0 "/Game/Assets/Materials/m_Player.m_Player")
        (Default|CustomCreate _asbp_master_unit)))
    (:then_2
      ;[1 1 1] Enemy Tokens Spawn
      (Utilities|Array|Shuffle (Variables|Default|Getn_Units_P2_Positions))
      (for _index_2 (range 0 (- (Variables|Default|Getn_Units_P2) 1))
        (bind _asbp_terrain_2 (Utilities|Casting|CastToBp_Terrain (Utilities|Array|Get(acopy) (Variables|Grid|GetActor_Tiles) (Utilities|Array|Get(acopy) (Variables|Default|Getn_Units_P2_Positions) _index_2))))
        (bind _returnvalue_3 (Game|SpawnActorfromClass "/Game/Blueprint/Bp_MasterUnit.Bp_MasterUnit_C" (Math|Transform|MakeTransform (Transformation|GetSocketLocation (Variables|/Game/Blueprint/Bp_Terrain.Bp_Terrain_C|GetStaticMesh _asbp_terrain_2) "Centro") "0, 0, 0" "1,1,1") "Undefined" 0 0))
        (bind _asbp_master_unit_2 (Utilities|Casting|CastToBp_MasterUnit _returnvalue_3))
        (Variables|/Game/Blueprint/Bp_MasterUnit.Bp_MasterUnit_C|SetTeam _asbp_master_unit_2 2)
        (Rendering|Material|SetMaterial (Variables|/Game/Blueprint/Bp_MasterUnit.Bp_MasterUnit_C|GetStaticMesh _asbp_master_unit_2) 0 "/Game/Assets/Materials/m_Enemy.m_Enemy")
        (Default|CustomCreate _asbp_master_unit_2)))
    (:then_3
      (Variables|Turns|SetTimer (Utilities|Time|GetGameTimeinSeconds)))))

(event EventTick
  (params (DeltaSeconds :type Float%20%28single-precision%29))
  (if (> (Utilities|Time|GetGameTimeinSeconds) (+ (Variables|Turns|GetTimer) (Variables|Turns|GetTimeToTurn)))
    (Variables|Turns|SetTimer (Utilities|Time|GetGameTimeinSeconds))
    (for _array_element (Variables|Grid|GetActor_Tiles)
      (bind _asbp_terrain (Utilities|Casting|CastToBp_Terrain _array_element))
      (Default|NextTurn _asbp_terrain))
    (Development|PrintString "Turno!!!" true true "(R=0.426688,G=1.000000,B=0.000000,A=1.000000)" 1.0)))

(fn ConstructionScript
  (bind _tiles (Variables|Grid|GetTiles))
  (bind _tiles_2 (Variables|Grid|GetTiles))
  (Utilities|FlowControl|Sequence
    (:then_0
      ;[1 1 1] Build Grid and setup Array
      (for _index (range 0 (Variables|Grid|Getx))
        (for _index_2 (range 0 (Variables|Grid|Gety))
          (bind _returnvalue (AddComponent|AddStaticMeshComponent false (Math|Transform|MakeTransform (Math|Vector|MakeVector (* _index 99.5) (+ (* _index_2 115.0) (Math|Float|SelectFloat 57.5 0.0 (== (Math|Integer|%(Integer) _index 2) 0))) 0.0) "0, 0, 0" "1,1,1")))
          (Utilities|Array|Add (Variables|Grid|GetTiles) _returnvalue))))
    (:then_1
      ;[1 1 1] Player 1 Spawn Table
      (for (_ _array_index) _tiles
        (if (<= _array_index (/ (Utilities|Array|Length _tiles) 2))
          (Utilities|Array|Add (Variables|Default|Getn_Units_P1_Positions) _array_index))))
    (:then_2
      ;[1 1 1] Player 2 Spawn Table
      (for (_ _array_index_2) _tiles_2
        (if (>= _array_index_2 (/ (Utilities|Array|Length _tiles_2) 2))
          (Utilities|Array|Add (Variables|Default|Getn_Units_P2_Positions) _array_index_2))))))