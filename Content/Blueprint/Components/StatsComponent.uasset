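; StatsComponent holds a character's stat block and run tallies: enemy deaths, damage per weapon and money.
; Update adds the difference between new and previous upgrade levels to each stat, then calls CallCallUptade.
; In that sum, the current area and projectile speed multipliers are crossed.
; AddMoney applies the money multiplier as a percentage bonus on the whole new total, not just the added amount.
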(event EventBeginPlay)

(event EventTick
  (params (DeltaSeconds :type Float%20%28single-precision%29)))

(fn Update
  (params (UpdateInfo :type Player%20Structure%20Structure) (PreviousLevel :type Player%20Structure%20Structure))
  (bind (_hpstructure _movespeedmultiplier _damagemultiplier _projectilespeedmultiplier _areamultiplier _projectilenumber _projectileduration _rateoffiremultiplier _luck _expmultiplier _moneymultiplier _pickarea _skips _discard _reroll _curse) (Utilities|Struct|BreakPlayerStructure UpdateInfo))
  (bind (_hpstructure_2 _movespeedmultiplier_2 _damagemultiplier_2 _projectilespeedmultiplier_2 _areamultiplier_2 _projectilenumber_2 _projectileduration_2 _rateoffiremultiplier_2 _luck_2 _expmultiplier_2 _moneymultiplier_2 _pickarea_2 _skips_2 _discard_2 _reroll_2 _curse_2) (Utilities|Struct|BreakPlayerStructure PreviousLevel))
  (Variables|Default|SetStructure (Utilities|Struct|MakePlayerStructure (Utilities|Struct|MakeHp_Structure (+ (- (.hpmax _hpstructure) (.hpmax _hpstructure_2)) (.hpmax (.hpstructure (Variables|Default|GetStructure)))) (+ (- (.currenthp _hpstructure) (.currenthp _hpstructure_2)) (.currenthp (.hpstructure (Variables|Default|GetStructure)))) (+ (- (.armor _hpstructure) (.armor _hpstructure_2)) (.armor (.hpstructure (Variables|Default|GetStructure)))) (+ (- (.recoveryhp _hpstructure) (.recoveryhp _hpstructure_2)) (.recoveryhp (.hpstructure (Variables|Default|GetStructure)))) (+ (- (.lifes _hpstructure) (.lifes _hpstructure_2)) (.lifes (.hpstructure (Variables|Default|GetStructure))))) (+ (- _movespeedmultiplier _movespeedmultiplier_2) (.movespeedmultiplier (Variables|Default|GetStructure))) (+ (- _damagemultiplier _damagemultiplier_2) (.damagemultiplier (Variables|Default|GetStructure))) (+ (- _projectilespeedmultiplier _projectilespeedmultiplier_2) (.areamultiplier (Variables|Default|GetStructure))) (+ (- _areamultiplier _areamultiplier_2) (.projectilespeedmultiplier (Variables|Default|GetStructure))) (+ (- _projectilenumber _projectilenumber_2) (.projectilenumber (Variables|Default|GetStructure))) (+ (- _projectileduration _projectileduration_2) (.projectileduration (Variables|Default|GetStructure))) (+ (- _rateoffiremultiplier _rateoffiremultiplier_2) (.rateoffiremultiplier (Variables|Default|GetStructure))) (+ (- _luck _luck_2) (.luck (Variables|Default|GetStructure))) (+ (- _expmultiplier _expmultiplier_2) (.expmultiplier (Variables|Default|GetStructure))) (+ (- _moneymultiplier _moneymultiplier_2) (.moneymultiplier (Variables|Default|GetStructure))) (+ (- _pickarea _pickarea_2) (.pickarea (Variables|Default|GetStructure))) (+ (- _skips _skips_2) (.skips (Variables|Default|GetStructure))) (+ (- _discard _discard_2) (.discard (Variables|Default|GetStructure))) (+ (- _reroll _reroll_2) (.reroll (Variables|Default|GetStructure))) (+ (- _curse _curse_2) (.curse (Variables|Default|GetStructure)))))
  (Default|CallCallUptade)
  (return true))

(fn AddEnemyDeath
  (Math|Integer|IncrementInt (Variables|Default|GetEnemyDeaths)
    (:%20%20
      (return true))))

(fn AddDamageStat
  (params (DamageToAdd :type Float%20%28double-precision%29%20%28by%20ref%29) (Weapon :type Data%20Table%20Object%20Reference%20%28by%20ref%29))
  (Utilities|Map|Add (Variables|Default|GetWeaponStats) Weapon (+ (.Value (Utilities|Map|Find (Variables|Default|GetWeaponStats) Weapon)) DamageToAdd))
  (return true))

(fn AddMoney
  (params (MoneyToAdd :type Float%20%28double-precision%29))
  (Variables|Default|SetMoney (+ (+ (Variables|Default|GetMoney) MoneyToAdd) (/ (* (+ (Variables|Default|GetMoney) MoneyToAdd) (Utilities|Struct|BreakPlayerStructure (Variables|Default|GetStructure))) 1e+02)))
  (return))