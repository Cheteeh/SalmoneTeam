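; Weapon inventory component that grants the player weapons and levels up those already owned.
; AddWeapon tracks a level per weapon in a map, either incrementing it and updating the live actor, or spawning a new one and recording its start time in the StatsComponent.
; Each weapon is keyed by its DataTable, with levels as row names.
; Spawned actors are attached to the player and cached for later updates.
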(fn AddWeapon
  (params (WeaponToAdd :type Data%20Table%20Object%20Reference))
  (bind _weaponslots (Variables|Default|GetWeaponSlots))
  (bind (_value _returnvalue) (Utilities|Map|Find _weaponslots WeaponToAdd))
  (if _returnvalue
    (Utilities|Map|Add (Variables|Default|GetWeaponSlots) WeaponToAdd (+ _value 1))
    (bind _success_ (CallFunction|UpdateWeapon WeaponToAdd (Utilities|String|StringToName (Utilities|String|ToString(Integer) _value))))
    (return _success_)
    (else
      (Utilities|Map|Add (Variables|Default|GetWeaponSlots) WeaponToAdd 1)
      (bind _success__2 (CallFunction|SpawnWeapon WeaponToAdd "1"))
      (Utilities|Map|Add (Variables|/Game/Blueprint/Components/StatsComponent.StatsComponent_C|GetWeaponTimer (Variables|Default|GetStatsComponent)) WeaponToAdd (Utilities|Time|GetTimeSeconds))
      (return _success__2))))

(fn SpawnWeapon
  (params (Weapon :type Data%20Table%20Object%20Reference) (Level :type Name))
  (bind _returnvalue (Utilities|GetDataTableRow Weapon Level)
    (:then
      (bind _returnvalue_2 (Game|SpawnActorfromClass (.Weapon (Utilities|Struct|BreakWeaponStructure _returnvalue)) (Math|Transform|MakeTransform (Transformation|GetActorLocation (Variables|Default|GetPlayerReference)) "0, 0, 0" "1.000000,1.000000,1.000000") "Undefined" 0 Weapon Level (Variables|Default|GetStatsComponent) 0))
      (Transformation|AttachActorToActor _returnvalue_2 (Variables|Default|GetPlayerReference) "None" "SnapToTarget" "SnapToTarget" "KeepRelative" true)
      (Utilities|Map|Add (Variables|Reference|GetWeaponSlotsReference) Weapon _returnvalue_2)
      (return true))))

(fn UpdateWeapon
  (params (Weapon :type Data%20Table%20Object%20Reference) (Level :type Name))
  (Default|UpdateWeapon (.Value (Utilities|Map|Find (Variables|Reference|GetWeaponSlotsReference) Weapon)) Level)
  (return true))