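; DropSystem is a component that spawns pickups from a drops data table when an enemy drops loot.
; EnemyDrop first rolls a drop chance boosted by the StatsComponent's Luck stat.
; On success, bosses roll a second Luck-boosted chance for a chest, falling back to 5XP, while regular enemies spawn 1XP or 5XP based on an XP enum.
; Only regular drops receive the row as ItemData; ObstacleDrop is an empty stub.
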(event EventBeginPlay)

(fn EnemyDrop
  (params (Boss :type Boolean) (XPDrop :type EnemyDrop_EN%20Enum :default "NewEnumerator0") (Location :type Vector))
  (bind _drop (CallFunction|CalcDropChanceEnemy))
  (if _drop
    (if Boss
      (bind _drop_2 (CallFunction|CalcBossChestProb))
      (if _drop_2
        (bind _returnvalue (Utilities|GetDataTableRow (Variables|Default|GetDrops_DT) "Chest")
          (:then
            (Game|SpawnActorfromClass :Class (Utilities|Struct|BreakItemDrop_ST _returnvalue) :SpawnTransform (Math|Transform|MakeTransform Location "0, 0, 0" "1.000000,1.000000,1.000000") :CollisionHandlingOverride "Undefined" :Instigator 0)))
        (else
          (bind _returnvalue_2 (Utilities|GetDataTableRow (Variables|Default|GetDrops_DT) "5XP")
            (:then
              (Game|SpawnActorfromClass :Class (Utilities|Struct|BreakItemDrop_ST _returnvalue_2) :SpawnTransform (Math|Transform|MakeTransform Location "0, 0, 0" "1.000000,1.000000,1.000000") :CollisionHandlingOverride "Undefined" :Instigator 0)))))
      (elif (Utilities|Enum|Equal(Enum) XPDrop "NewEnumerator5")
        (bind _returnvalue_3 (Utilities|GetDataTableRow (Variables|Default|GetDrops_DT) "5XP")
          (:then
            (Game|SpawnActorfromClass (Utilities|Struct|BreakItemDrop_ST _returnvalue_3) (Math|Transform|MakeTransform Location "0, 0, 0" "1.000000,1.000000,1.000000") "Undefined" 0 "None" _returnvalue_3 0)))
        (else
          (bind _returnvalue_4 (Utilities|GetDataTableRow (Variables|Default|GetDrops_DT) "1XP")
            (:then
              (Game|SpawnActorfromClass (Utilities|Struct|BreakItemDrop_ST _returnvalue_4) (Math|Transform|MakeTransform Location "0, 0, 0" "1.000000,1.000000,1.000000") "Undefined" 0 "None" _returnvalue_4 0))))))))

(fn CalcDropChanceEnemy
  (if (< (Math|Random|RandomFloatinRange 0.0 1e+02) (+ (Variables|Default|GetDropChance) (Utilities|Struct|BreakPlayerStructure (Variables|/Game/Blueprint/Components/StatsComponent.StatsComponent_C|GetStructure (Variables|Default|GetStatsComponent)))))
    (return true)
    (else
      (return false))))

(fn CalcBossChestProb
  (if (< (Math|Random|RandomFloatinRange 0.0 1e+02) (+ (Variables|Default|GetDropChanceChest) (Utilities|Struct|BreakPlayerStructure (Variables|/Game/Blueprint/Components/StatsComponent.StatsComponent_C|GetStructure (Variables|Default|GetStatsComponent)))))
    (return true)
    (else
      (return false))))

(fn ObstacleDrop)