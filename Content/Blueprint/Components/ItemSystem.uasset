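; Item system component that tracks the passive items held and their levels, and applies their stats.
; AddItem inserts an item at level 1 or raises its level in the PasiveSlots map, while QueryItem reports presence and level.
; Each item is its own DataTable with rows named by level.
; UpdateStats passes the new row, plus the previous one on upgrades, to StatsComponent.
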(fn AddItem
  (params (Item :type Data%20Table%20Object%20Reference))
  (bind _pasiveslots (Variables|Default|GetPasiveSlots))
  (bind (_value _returnvalue) (Utilities|Map|Find _pasiveslots Item))
  (if _returnvalue
    (Utilities|Map|Add (Variables|Default|GetPasiveSlots) Item (+ _value 1))
    (bind _success_ (CallFunction|UpdateStats Item (Utilities|String|StringToName (Utilities|String|ToString(Integer) _value)) (Utilities|String|StringToName (Utilities|String|ToString(Integer) (- _value 1))) false))
    (if _success_
      (return true)
      (else
        (Development|PrintString "Item No encontrado")))
    (else
      (Utilities|Map|Add (Variables|Default|GetPasiveSlots) Item 1)
      (bind _success__2 (CallFunction|UpdateStats Item "1" "None" true))
      (if _success__2
        (return true)
        (else
          (Development|PrintString "Item No encontrado"))))))

(fn QueryItem
  (params (Item :type Data%20Table%20Object%20Reference))
  (bind _pasiveslots (Variables|Default|GetPasiveSlots))
  (bind (_value _returnvalue) (Utilities|Map|Find _pasiveslots Item))
  (if _returnvalue
    (return true _value)
    (else
      (return false 0))))

(fn UpdateStats
  (params (Item :type Data%20Table%20Object%20Reference) (Level :type Name) (PreviusLevel :type Name) (Newitem? :type Boolean))
  (if Newitem?
    (bind _returnvalue (Utilities|GetDataTableRow Item Level)
      (:then
        (bind _success_ (Default|Update (Variables|Default|GetStatsComponent) (.Structure (Utilities|Struct|BreakItemStructure _returnvalue))))
        (return _success_))
      (:RowNotFound
        (return false)))
    (else
      (bind _returnvalue_2 (Utilities|GetDataTableRow Item Level)
        (:then
          (bind _returnvalue_3 (Utilities|GetDataTableRow Item PreviusLevel)
            (:then
              (bind _success__2 (Default|Update (Variables|Default|GetStatsComponent) (.Structure (Utilities|Struct|BreakItemStructure _returnvalue_2)) (.Structure (Utilities|Struct|BreakItemStructure _returnvalue_3))))
              (return _success__2))))))))