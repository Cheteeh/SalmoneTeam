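; Spawner component that runs timed enemy waves around the player, loading each wave's enemy mix, alive cap and spawn rate from a level data table.
; After a short delay, timers advance the wave every minute and spawn every second.
; Each tick splits the batch, capped by free slots, evenly across player-relative boxes.
; Enemy types are picked by weighted random, then spawned as Enemy actors configured from the EnemyList table.
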(event Custom|Initialite
  ;[0 0 0] Iniciamos el timer para las wave
  (Utilities|Time|SetTimerbyFunctionName 0 "InitialiteWave" 6e+01 true)
  (Utilities|Time|SetTimerbyFunctionName 0 "SpawnWave" 1.0 true)
  (CallFunction|InitialiteWave)
  (CallFunction|SpawnWave))

(event EventBeginPlay
  (Utilities|Time|SetTimerbyEvent (delegate Custom|Initialite) 1.0))

(fn SpawnEnemy
  (params (Position :type Vector) (Name :type Name))
  (bind (_x _y) (Class|KismetMathLibrary|BreakVector3f Position))
  (bind _playerreference (Variables|Reference|GetPlayerReference))
  (bind _returnvalue (Utilities|GetDataTableRow "/Game/Blueprint/Data/Datatables/EnemyList.EnemyList" Name)
    (:then
      (Game|SpawnActorfromClass :Class "/Game/Blueprint/Actors/Enemy.Enemy_C" :SpawnTransform (Math|Transform|MakeTransform (Math|Vector|MakeVector _x _y 5e+01) "0, 0, 0" "1.000000,1.000000,1.000000") :CollisionHandlingOverride "AdjustIfPossibleButAlwaysSpawn" :Target _playerreference :PlayerStatsComponent (Variables|/Game/Blueprint/Actors/PlayerUnit.PlayerUnit_C|GetStatsComponent _playerreference) :DT_EnemyStructure _returnvalue :SpawnSystem self :Instigator 0)
      (Math|Integer|IncrementInt (Variables|Controladores|GetEnemyAmountInPlay)
        (:%20%20
          (return true))))))

(fn SpawnPositionCalc
  (params (Spawner :type Vector))
  (return (+ (Transformation|GetActorLocation (Variables|Reference|GetPlayerReference)) Spawner)))

(fn InitialiteWave
  (bind _result (Math|Integer|IncrementInt (Variables|Controladores|GetWaveCounter))
    (:%20%20
      ;[0 0 0 1 10] Leer de una tabla la wave y configurar el spawn
      (bind _returnvalue (Utilities|GetDataTableRow (Variables|Default|GetLevel_DataTable) (Utilities|String|StringToName (Utilities|String|ToString(Integer) _result)))
        (:then
          (Variables|Default|SetList%20Of%20Enemies (.enemies (Utilities|Struct|BreakST_LevelStructure _returnvalue)))
          (Variables|Default|SetMaxEnemiesInGame (.maxenemiesinwave (Utilities|Struct|BreakST_LevelStructure _returnvalue)))
          (Variables|Default|SetRateOfSpawn (.rateofspawn (Utilities|Struct|BreakST_LevelStructure _returnvalue))))
        (:RowNotFound
          (Development|PrintString "Horror"))))))

(fn SpawnWave
  (bind _enemyamountinplay (Variables|Controladores|GetEnemyAmountInPlay))
  (bind _maxenemiesingame (Variables|Default|GetMaxEnemiesInGame))
  (bind _rateofspawn (Variables|Default|GetRateOfSpawn))
  (bind _returnvalue (- _maxenemiesingame _enemyamountinplay))
  (if (< (Variables|Controladores|GetEnemyAmountInPlay) (Variables|Default|GetMaxEnemiesInGame))
    (LocalVariables|SetEnemiesToSpawn (/ (Math|Integer|SelectInt _rateofspawn _returnvalue (> _returnvalue _rateofspawn)) (+ (Utilities|Array|LastIndex (Variables|Default|GetSpawnPoints)) 1)))
    (for _array_element (Variables|Default|GetSpawnPoints)
      (for _index (range 1 (LocalVariables|GetEnemiesToSpawn))
        (bind _enemytospawn (CallFunction|CalcEnemytoSpawn (Variables|Default|GetList%20Of%20Enemies)))
        (bind _spawnposition (CallFunction|SpawnPositionCalc (Math|Random|RandomPointinBoundingBox (.Origin (Math|BoxSphereBounds|BreakBoxSphereBounds _array_element)) (.BoxExtent (Math|BoxSphereBounds|BreakBoxSphereBounds _array_element)))))
        (CallFunction|SpawnEnemy _spawnposition _enemytospawn)))))

(fn CalcEnemytoSpawn
  (params (ListOfEnemies :type Map%20of%20Names%20to%20Integers))
  (LocalVariables|SetTotal 1)
  (LocalVariables|SetControlador 1)
  (bind _values (Utilities|Map|Values ListOfEnemies))
  (for _array_element _values
    (LocalVariables|SetTotal (+ (LocalVariables|GetTotal) _array_element)))
  (LocalVariables|SetGanador (Math|Random|RandomIntegerinRange (LocalVariables|GetControlador) (LocalVariables|GetTotal)))
  (bind _values_2 (Utilities|Map|Values ListOfEnemies))
  (bind (_array_element_2 _array_index) (Utilities|Array|ForEachLoopwithBreak _values_2 :!label _label)
    (:LoopBody
      (if (>= (+ (LocalVariables|GetControlador) _array_element_2) (LocalVariables|GetGanador))
        (LocalVariables|SetIndex _array_index)
        (goto _label Break)
        (else
          (LocalVariables|SetControlador (+ (LocalVariables|GetControlador) _array_element_2)))))
    (:Completed
      (bind _keys (Utilities|Map|Keys ListOfEnemies))
      (return (Utilities|Array|Get(acopy) _keys (LocalVariables|GetIndex))))))