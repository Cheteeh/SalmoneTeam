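; Health component that applies damage, healing and periodic HP recovery to the HP structure held in a StatsComponent.
; ApplyDamage subtracts flat armor, clamps HP at zero and returns damage dealt and death state, while Heal caps at max HP.
; CheckRecovery starts a one-time-guarded, looping one-second timer that heals by the recovery stat.
; Initialize binds to the stats update dispatcher but is disconnected from BeginPlay.
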(event EventBeginPlay)

(fn ApplyDamage
  (params (DamageToDeal :type Float%20%28double-precision%29))
  (bind _damage_output (CallFunction|Armor DamageToDeal))
  (if (<= _damage_output 0.0)
    ;[1 1 1] Añadir Feedback de no DAÑO
    (return false 0.0)
    (else
      ;[1 1 1] Aplicamos el daño
      (if (> (- (.currenthp (.HpStructure (Utilities|Struct|BreakPlayerStructure (Variables|/Game/Blueprint/Components/StatsComponent.StatsComponent_C|GetStructure (Variables|Default|GetStatsComponent))))) _damage_output) 0.0)
        (Utilities|Struct|SetmembersinHp_Structure (.HpStructure (Utilities|Struct|BreakPlayerStructure (Variables|/Game/Blueprint/Components/StatsComponent.StatsComponent_C|GetStructure (Variables|Default|GetStatsComponent)))) (- (.currenthp (.HpStructure (Utilities|Struct|BreakPlayerStructure (Variables|/Game/Blueprint/Components/StatsComponent.StatsComponent_C|GetStructure (Variables|Default|GetStatsComponent))))) _damage_output))
        (return false _damage_output)
        (else
          ;[1 1 1] Si ha muerto se devuelte True
          (Utilities|Struct|SetmembersinHp_Structure (.HpStructure (Utilities|Struct|BreakPlayerStructure (Variables|/Game/Blueprint/Components/StatsComponent.StatsComponent_C|GetStructure (Variables|Default|GetStatsComponent)))) 0.0)
          (return true _damage_output))))))

(fn Heal
  (params (HpToHeal :type Float%20%28double-precision%29))
  (bind _statscomponent (Variables|Default|GetStatsComponent))
  (bind _statscomponent_2 (Variables|Default|GetStatsComponent))
  (bind _structure (Variables|/Game/Blueprint/Components/StatsComponent.StatsComponent_C|GetStructure _statscomponent))
  (bind _structure_2 (Variables|/Game/Blueprint/Components/StatsComponent.StatsComponent_C|GetStructure _statscomponent_2))
  (bind _hpstructure (Utilities|Struct|BreakPlayerStructure _structure))
  (bind _hpstructure_2 (Utilities|Struct|BreakPlayerStructure _structure_2))
  (bind _returnvalue (+ HpToHeal (.currenthp _hpstructure)))
  (if (> _returnvalue (.hpmax _hpstructure))
    (Utilities|Struct|SetmembersinHp_Structure _hpstructure_2 (.HpMax (Utilities|Struct|BreakHp_Structure _hpstructure_2)))
    (else
      (Utilities|Struct|SetmembersinHp_Structure (.HpStructure (Utilities|Struct|BreakPlayerStructure (Variables|/Game/Blueprint/Components/StatsComponent.StatsComponent_C|GetStructure (Variables|Default|GetStatsComponent)))) _returnvalue))))

(fn CheckRecovery
  (if (not (Variables|Default|GetRecoveryController))
    (if (> (.recoveryhp (.HpStructure (Utilities|Struct|BreakPlayerStructure (Variables|/Game/Blueprint/Components/StatsComponent.StatsComponent_C|GetStructure (Variables|Default|GetStatsComponent))))) 0.0)
      (bind _returnvalue (Utilities|Time|SetTimerbyFunctionName 0 "Recovery" 1.0 true))
      (Variables|Default|SetRecoveryTimer _returnvalue)
      (Variables|Default|SetRecoveryController true)
      (return))))

(fn Recovery
  (bind _statscomponent (Variables|Default|GetStatsComponent))
  (bind _structure (Variables|/Game/Blueprint/Components/StatsComponent.StatsComponent_C|GetStructure _statscomponent))
  (bind _hpstructure (Utilities|Struct|BreakPlayerStructure _structure))
  (if (< (.currenthp _hpstructure) (.hpmax _hpstructure))
    (CallFunction|Heal (.RecoveryHp (Utilities|Struct|BreakHp_Structure (.HpStructure (Utilities|Struct|BreakPlayerStructure (Variables|/Game/Blueprint/Components/StatsComponent.StatsComponent_C|GetStructure (Variables|Default|GetStatsComponent)))))))))

(fn Armor
  (params (DamageInput :type Float%20%28double-precision%29))
  (bind _statscomponent (Variables|Default|GetStatsComponent))
  (bind _structure (Variables|/Game/Blueprint/Components/StatsComponent.StatsComponent_C|GetStructure _statscomponent))
  (bind _hpstructure (Utilities|Struct|BreakPlayerStructure _structure))
  (bind _armor (Utilities|Struct|BreakHp_Structure _hpstructure))
  (bind _returnvalue (- DamageInput _armor))
  (if (> _armor 0.0)
    (return (Math|Float|SelectFloat 0.0 _returnvalue (<= _returnvalue 0.0)))
    (else
      (return DamageInput))))

(fn Initialize
  (EventDispatchers|BindEventtoCallUptade (Variables|Default|GetStatsComponent) (EventDispatchers|CreateEvent :!event CheckRecovery))
  (return))