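; Game instance for a two-team tactics game that tracks turn ownership and a chip bag of units for each team.
; GenerateChipBags sorts every Bp_MasterUnit actor in the level into the Team 0 or Team 1 bag, then prints both for debugging.
; NextTurnEvent calls NextTurn, which flips TurnOwner between the teams, copies it to the PC_Tactics controller's Team and prints whose turn it is.
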(event Custom|NextTurnEvent
  (CallFunction|NextTurn))

(event Custom|GenerateChipBags
  (bind _outactors (Actor|GetAllActorsOfClass "/Game/Blueprint/Bp_MasterUnit.Bp_MasterUnit_C"))
  (for _array_element _outactors
    (if (== (Variables|/Game/Blueprint/Bp_MasterUnit.Bp_MasterUnit_C|GetTeam _array_element) 0)
      (Utilities|Array|Add (Variables|Default|GetTeam0_ChipsBag) _array_element)
      (else
        (Utilities|Array|Add (Variables|Default|GetTeam1_ChipsBag) _array_element))))
  ;[1 0.4227 0.01201] Debug
  (Development|PrintString "Team o Chips Bag:" true true "(R=0.399979,G=0.000000,B=0.572917,A=1.000000)" 1e+01)
  (for _array_element_2 (Variables|Default|GetTeam0_ChipsBag)
    (Development|PrintString (Utilities|GetDisplayName _array_element_2) true true "(R=1.000000,G=0.000000,B=0.049778,A=1.000000)" 1e+01))
  (Development|PrintString "Team 1 Chips Bag:" true true "(R=0.399979,G=0.000000,B=0.572917,A=1.000000)" 1e+01)
  (for _array_element_3 (Variables|Default|GetTeam1_ChipsBag)
    (Development|PrintString (Utilities|GetDisplayName _array_element_3) true true "(R=1.000000,G=0.000000,B=0.049778,A=1.000000)" 1e+01)))

(fn NextTurn
  (bind _aspc_tactics (Utilities|Casting|CastToPC_Tactics (Game|GetPlayerController 0)))
  (if (== (Variables|Default|GetTurnOwner) 0)
    (bind _output_get (Variables|Default|SetTurnOwner 1))
    (Variables|/Game/Blueprint/PC_Tactics.PC_Tactics_C|SetTeam _aspc_tactics _output_get)
    (else
      (bind _output_get_2 (Variables|Default|SetTurnOwner 0))
      (Variables|/Game/Blueprint/PC_Tactics.PC_Tactics_C|SetTeam _aspc_tactics _output_get_2)))
  (Development|PrintString (Utilities|String|Append "Team's Turn: " (Utilities|String|ToString(Integer) (Variables|Default|GetTurnOwner))) true true "(R=1.000000,G=0.000000,B=0.007180,A=1.000000)" 1e+01))