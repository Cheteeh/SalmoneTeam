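; Base projectile actor that damages actors implementing the Vampire_Interaction interface when its collision overlaps them.
; The construction script sets the movement component's initial speed from ProjectileSpeed, and BeginPlay starts a one-shot lifetime timer using Duration.
; On a valid hit it sends damage through the interface, records it in PlayerStats under the instigating weapon, and destroys itself only if the target returns true.
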(event OnComponentBeginOverlap(Collision)
  (params (OverlappedComponent :type Primitive%20Component%20Object%20Reference) (OtherActor :type Actor%20Object%20Reference) (OtherComp :type Primitive%20Component%20Object%20Reference) (OtherBodyIndex :type Integer) (bFromSweep :type Boolean) (SweepResult :type Hit%20Result%20Structure%20%28by%20ref%29))
  (bind _hitactor (Collision|BreakHitResult SweepResult))
  ;[1 1 1] Comprueba si colsiona contra algun actor con la interfaz integrada
  (if (Utilities|DoesObjectImplementInterface _hitactor "/Game/Blueprint/ManagersAndControllers/Vampire_Interaction.Vampire_Interaction_C")
    ;[1 1 1] Manda la informacion de daño al objeto
    (bind _success_ (Class|VampireInteraction|DamageInterface(Message) _hitactor (Variables|Default|GetDamage)))
    (Default|AddDamageStat (Variables|Default|GetPlayerStats) (Variables|Default|GetDamage) (Variables|Default|GetWeaponInstigator))
    ;[1 1 1] Destruye el objeto si recibe el True del objeto que impacta
    (if _success_
      (Actor|DestroyActor))))

(event Custom|KillProjectile
  (Actor|DestroyActor))

(event EventBeginPlay
  (Utilities|Time|SetTimerbyEvent (EventDispatchers|CreateEvent :!event Custom|KillProjectile) (Variables|Default|GetDuration)))

(fn ConstructionScript
  (Variables|/Script/Engine.ProjectileMovementComponent|SetInitialSpeed (Variables|Default|GetProjectileMovement) (Variables|Default|GetProjectileSpeed)))