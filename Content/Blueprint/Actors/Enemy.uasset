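; Enemy actor for a Vampire Survivors-style game that takes material, HP, damage and speed from DTEnemyStructure and chases Target with AIMoveTo.
; Sphere overlap with the player starts looping timed damage; end overlap nulls the damaged actor without clearing the timer.
; Incoming damage goes through HpSystem with floating text; death records the kill, triggers DropSystem and destroys the enemy.
; A periodic check culls distant enemies, decrementing the SpawnSystem count as death does.
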(event OnComponentBeginOverlap(Sphere)
  (params (OverlappedComponent :type Primitive%20Component%20Object%20Reference) (OtherActor :type Actor%20Object%20Reference) (OtherComp :type Primitive%20Component%20Object%20Reference) (OtherBodyIndex :type Integer) (bFromSweep :type Boolean) (SweepResult :type Hit%20Result%20Structure%20%28by%20ref%29))
  ;[0 0 0] Funcion de daño al player cuando colisiona con el
  (if (== (Utilities|GetClass OtherActor) "/Game/Blueprint/Actors/PlayerUnit.PlayerUnit_C")
    (if (Utilities|DoesObjectImplementInterface OtherActor "/Game/Blueprint/ManagersAndControllers/Vampire_Interaction.Vampire_Interaction_C")
      (Variables|Default|SetActorToDamage OtherActor)
      (bind _returnvalue (Utilities|Time|SetTimerbyEvent (delegate Custom|CustomEvent_0) 0.25 true))
      (Variables|Default|SetTimerToDamage _returnvalue))))

(event OnComponentEndOverlap(Sphere)
  (params (OverlappedComponent :type Primitive%20Component%20Object%20Reference) (OtherActor :type Actor%20Object%20Reference) (OtherComp :type Primitive%20Component%20Object%20Reference) (OtherBodyIndex :type Integer))
  ;[0 0 0] Desactiva el Dot al player
  (if (== (Utilities|GetClass OtherActor) "/Game/Blueprint/Actors/PlayerUnit.PlayerUnit_C")
    (if (Utilities|DoesObjectImplementInterface OtherActor "/Game/Blueprint/ManagersAndControllers/Vampire_Interaction.Vampire_Interaction_C")
      (Variables|Default|SetActorToDamage 0)
      (Utilities|Time|UnpauseTimerbyHandle (Variables|Default|GetTimerToDamage)))))

(event Custom|CustomEvent_0
  ;[0 0 0] Funcion de daño al player cuando colisiona con el
  (Class|VampireInteraction|DamagetoPlayer(Message) (Variables|Default|GetActorToDamage) (Variables|Default|GetDamageDealt_0)))

(event EventBeginPlay
  (bind _dt_enemystructure (Variables|Default|GetDT_EnemyStructure))
  (bind (_enemyname _hp _damage _speed _boss _xpdrop _material) (Utilities|Struct|BreakEnemyStructure _dt_enemystructure))
  ;[1 1 1] Seteo de Valores e inicio de la IA sencilla para perseguir al player
  (Rendering|Material|SetMaterial (Variables|GetMeshComponent) 0 _material)
  (Utilities|Struct|SetmembersinHp_Structure (.HpStructure (Utilities|Struct|BreakPlayerStructure (Variables|/Game/Blueprint/Components/StatsComponent.StatsComponent_C|GetStructure (Variables|Default|GetStatsComponent)))) _hp)
  (Variables|Default|SetDamageDealt_0 _damage)
  (Variables|Default|SetSpeed _speed)
  (AI|AIMoveTo (AI|GetAIController (Pawn|GetController)) "0, 0, 0" (Variables|Default|GetTarget) 0.0 "Disable" "Disable" false true true "Disable"
    (:then
      (Utilities|Time|SetTimerbyFunctionName 0 "CheckDistancePlayer" 5.0 true))))

(fn ConstructionScript
  (Variables|/Game/Blueprint/Components/Hp_System.Hp_System_C|SetStatsComponent (Variables|Default|GetHp_System) (Variables|Default|GetStatsComponent))
  (Variables|/Game/Blueprint/Components/DropSystem.DropSystem_C|SetStatsComponent (Variables|Default|GetDropSystem) (Variables|Default|GetPlayerStatsComponent)))

(fn Dead
  (params (Drop? :type Boolean))
  (bind _dt_enemystructure (Variables|Default|GetDT_EnemyStructure))
  (Default|AddEnemyDeath (Variables|Default|GetPlayerStatsComponent))
  ;[1 1 1] *** Añadir logica para el drop de XP
  (Default|EnemyDrop (Variables|Default|GetDropSystem) (.boss _dt_enemystructure) (.xpdrop _dt_enemystructure) (Transformation|GetActorLocation))
  ;[0 0 0 1 10] Eliminamos el enemigo del controlador
  (Math|Integer|DecrementInt (Variables|/Game/Blueprint/Components/SpawnerComponent.SpawnerComponent_C|GetEnemyAmountInPlay (Variables|Default|GetSpawnSystem))
    (:%20%20
      (Actor|DestroyActor))))

(fn CheckDistancePlayer
  (if (> (Transformation|GetDistanceTo (Variables|Default|GetTarget) self) 3.5e+03)
    ;[0 0 0 1 10] Eliminamos el enemigo del controlador
    (Math|Integer|DecrementInt (Variables|/Game/Blueprint/Components/SpawnerComponent.SpawnerComponent_C|GetEnemyAmountInPlay (Variables|Default|GetSpawnSystem))
      (:%20%20
        (Actor|DestroyActor)))))

(fn DamageInterface
  (params (Damage :type Float%20%28double-precision%29))
  (bind _returnvalue (Transformation|GetActorLocation))
  (bind _returnvalue_2 (Transformation|GetActorLocation))
  ;[1 1 1] Applicamos el daño del jugador al enemigo
  (bind _dead_ (Default|ApplyDamage (Variables|Default|GetHp_System) Damage))
  ;[1 1 1] Añadimos el floating Damage Text
  (if _dead_
    (Game|SpawnActorfromClass "/Game/Blueprint/Interfaz/Bp_FloatingText.Bp_FloatingText_C" (Math|Transform|MakeTransform (Math|Vector|MakeVector (.x _returnvalue) (.y _returnvalue) (+ (.z _returnvalue) 4e+01)) "0, 0, 0" "1.000000,1.000000,1.000000") "AlwaysSpawn" 0 Damage (Math|Color|MakeColor 0 0 255) 0)
    ;[1 1 1] Destruimos la unidad
    (CallFunction|Dead false)
    (else
      (Game|SpawnActorfromClass "/Game/Blueprint/Interfaz/Bp_FloatingText.Bp_FloatingText_C" (Math|Transform|MakeTransform (Math|Vector|MakeVector (.x _returnvalue_2) (.y _returnvalue_2) (+ (.z _returnvalue_2) 4e+01)) "0, 0, 0" "1.000000,1.000000,1.000000") "AlwaysSpawn" 0 Damage "(B=0,G=0,R=0,A=0)" 0)))
  (return true))

(fn DamagetoPlayer
  (params (DamageToPlayer :type Float%20%28double-precision%29))
  ;[1 1 1] Pasamos el daño que causa al player el enemigo
)

(fn MagnetMode
  (params (PlayerReference :type Player%20Unit%20Object%20Reference))
  ;[1 1 1] No se usa
)