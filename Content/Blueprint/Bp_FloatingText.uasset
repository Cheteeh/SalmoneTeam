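; Floating damage number actor that shows a DamageText value on a TextRender component, rounded up to a whole number.
; The text is set in both the construction script and BeginPlay.
; On BeginPlay a timeline drives the text's X and Y scale, and the actor destroys itself when the timeline finishes.
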(event EventTick
  (params (DeltaSeconds :type Float%20%28single-precision%29)))

(event EventBeginPlay
  (Rendering|Components|TextRender|SetText (Variables|Default|GetTextRender) (Utilities|Text|ToText(Integer) (Math|Float|Ceil (Variables|Default|GetDamageText))))
  (bind _scale (Timeline|Timeline_0 Play)
    (:Update
      (Rendering|Components|TextRender|SetXScale (Variables|Default|GetTextRender) _scale)
      (Rendering|Components|TextRender|SetYScale (Variables|Default|GetTextRender) _scale))
    (:Finished
      (Actor|DestroyActor))))

(fn ConstructionScript
  (Rendering|Components|TextRender|SetText (Variables|Default|GetTextRender) (Utilities|Text|ToText(Integer) (Math|Float|Ceil (Variables|Default|GetDamageText)))))