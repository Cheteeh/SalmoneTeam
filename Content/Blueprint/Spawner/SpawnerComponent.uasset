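; Spawner component that runs timed enemy waves, placing groups at random points inside spawn boxes offset from the player's location.
; BeginPlay starts a looping wave timer and the first wave, whose own timer spawns groups until the SpawnWaves countdown reaches zero.
; Each group reads its data table row by wave number, splitting the amount across spawn points.
; SpawnEnemy currently only prints a debug string; its actor spawn is disconnected.
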(event Custom|EventWave
  (Math|Integer|IncrementInt (Variables|Controladores|GetWaveCounter)
    (:%20%20
      (bind _returnvalue (Utilities|Time|SetTimerbyEvent (delegate Custom|SpawnInWave) (Math|Conversions|ToFloat(Integer) (/ 60 (Variables|Controladores|GetSpawnWaves))) true))
      (Variables|Controladores|SetSpawnEnemiesTimer _returnvalue)
      (CallFunction|SpawninWave))))

(event Custom|SpawnInWave
  (if (== (Variables|Controladores|GetSpawnWaves) 0)
    (Utilities|Time|PauseTimerbyHandle (Variables|Controladores|GetSpawnEnemiesTimer))
    (else
      (CallFunction|SpawnGroupOfEnemies (Variables|Controladores|GetWaveCounter))
      (Math|Integer|DecrementInt (Variables|Controladores|GetSpawnWaves)))))

(event EventBeginPlay
  ;[0 0 0] Iniciamos el timer para las wave
  (Utilities|FlowControl|Delay 0.1)
  (bind _returnvalue (Utilities|Time|SetTimerbyEvent (EventDispatchers|CreateEvent :!event Custom|EventWave) 6e+01 true))
  (Variables|Referemce|SetWaveTimer _returnvalue)
  (CallFunction|EventWave))

(fn SpawnEnemy
  (params (Position :type Vector) (DT_EnemyStructure :type Enemy%20Structure%20Structure))
  (Development|PrintString "Enemy")
  (return true))

(fn SpawnPositionCalc
  (params (Spawner :type Vector))
  (return (+ (Transformation|GetActorLocation (Variables|Referemce|GetPlayerReference)) Spawner)))

(fn SpawnGroupOfEnemies
  (params (Wave :type Integer))
  (bind _returnvalue (Utilities|GetDataTableRow (Variables|Default|GetData%20Table) (Utilities|String|StringToName (Utilities|String|ToString(Integer) Wave)))
    (:then
      (LocalVariables|SetEnemiesPerSpawnPoint (/ (.Amount (Utilities|Struct|BreakSpawnStructure _returnvalue)) (+ (Utilities|Array|LastIndex (Variables|Default|GetSpawnPoints)) 1)))
      (for _array_element (Variables|Default|GetSpawnPoints)
        (for _index (range 1 (LocalVariables|GetEnemiesPerSpawnPoint))
          (bind _spawnposition (CallFunction|SpawnPositionCalc (Math|Random|RandomPointinBoundingBox (.Origin (Math|BoxSphereBounds|BreakBoxSphereBounds _array_element)) (.BoxExtent (Math|BoxSphereBounds|BreakBoxSphereBounds _array_element)))))
          (CallFunction|SpawnEnemy _spawnposition (.Enemy (Utilities|Struct|BreakSpawnStructure _returnvalue))))))))