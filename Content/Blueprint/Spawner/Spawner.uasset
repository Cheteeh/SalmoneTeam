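; Enemy spawner actor that follows a Target actor and spawns enemies at its Spawner component, passing that Target to each.
; Every tick it moves to the Target, and AddEnemy increments UnitsToSpawn on a timed interval, then immediately calls SpawnEnemy, which decrements it.
; Spawner overlap events toggle CanSpawn, which no graph reads, and ending an overlap loops SpawnEnemy until UnitsToSpawn is used up.
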(event OnComponentBeginOverlap(Spawner)
  (params (OverlappedComponent :type Primitive%20Component%20Object%20Reference) (OtherActor :type Actor%20Object%20Reference) (OtherComp :type Primitive%20Component%20Object%20Reference) (OtherBodyIndex :type Integer) (bFromSweep :type Boolean) (SweepResult :type Hit%20Result%20Structure%20%28by%20ref%29))
  (Variables|Default|SetCanSpawn? false))

(event OnComponentEndOverlap(Spawner)
  (params (OverlappedComponent :type Primitive%20Component%20Object%20Reference) (OtherActor :type Actor%20Object%20Reference) (OtherComp :type Primitive%20Component%20Object%20Reference) (OtherBodyIndex :type Integer))
  (Variables|Default|SetCanSpawn? true)
  (if (> (Variables|Default|GetUnitsToSpawn) 0) :!label _label
    (CallFunction|SpawnEnemy)
    (goto _label)))

(event EventTick
  (params (DeltaSeconds :type Float%20%28single-precision%29))
  (Transformation|SetActorLocation (Transformation|GetActorLocation (Variables|Default|GetTarget)) false false)
  (CallFunction|AddEnemy))

(fn ConstructionScript)

(fn AddEnemy
  (bind _returnvalue (Utilities|Time|GetGameTimeinSeconds))
  (if (>= _returnvalue (Variables|Default|GetTime))
    (Variables|Default|SetTime (+ (Variables|Default|GetTimer) _returnvalue))
    (Variables|Default|SetUnitsToSpawn (+ (Variables|Default|GetUnitsToSpawn) 1))
    (CallFunction|SpawnEnemy)))

(fn SpawnEnemy
  (Game|SpawnActorfromClass :Class "/Game/Blueprint/Spawner/Enemy.Enemy_C" :SpawnTransform (Math|Transform|MakeTransform (Transformation|GetWorldLocation (Variables|Default|GetSpawner)) "0, 0, 0" "1.000000,1.000000,1.000000") :CollisionHandlingOverride "Undefined" :Target (Variables|Default|GetTarget) :Instigator 0)
  (Variables|Default|SetUnitsToSpawn (- (Variables|Default|GetUnitsToSpawn) 1)))