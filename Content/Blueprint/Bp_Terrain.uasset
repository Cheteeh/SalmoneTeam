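; Board tile for a turn-based territory game, tracking an owning team and a point count shown on its widget.
; On BeginPlay it caches neighboring tiles with a sphere overlap.
; Each Next_Turn, an overlapping unit claims, reinforces or weakens it, then full encirclement by user tiles favors the player.
; Every fifth turn, strong AI tiles spread, reinforcing allies, weakening user tiles and capturing neutral neighbors.
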(event OnComponentBeginOverlap(Box)
  (params (OverlappedComponent :type Primitive%20Component%20Object%20Reference) (OtherActor :type Actor%20Object%20Reference) (OtherComp :type Primitive%20Component%20Object%20Reference) (OtherBodyIndex :type Integer) (bFromSweep :type Boolean) (SweepResult :type Hit%20Result%20Structure%20%28by%20ref%29))
  (Variables|Default|SetEstaOcupada? true)
  (Variables|Default|SetQuienMeocupa OtherActor))

(event OnComponentEndOverlap(Box)
  (params (OverlappedComponent :type Primitive%20Component%20Object%20Reference) (OtherActor :type Actor%20Object%20Reference) (OtherComp :type Primitive%20Component%20Object%20Reference) (OtherBodyIndex :type Integer))
  (Variables|Default|SetEstaOcupada? false))

(event Custom|GhostTileOFF)

(event Custom|GhostTileOn)

(event Custom|Next_Turn
  (Variables|Turns|SetTurnCounter (CallFunction|PlusOne(Int) (Variables|Turns|GetTurnCounter)))
  (CallFunction|CheckTokeninTerrain)
  (CallFunction|Surrounded)
  (if (CallFunction|EqualsZero(Int) (Math|Integer|%(Integer) (Variables|Turns|GetTurnCounter) 5))
    (CallFunction|Spread)))

(event Custom|Tiles
  ;[1 1 1] Seteo las casilla que hay alrededor
  (CallFunction|TilesatRange))

(event EventBeginPlay
  ;[1 1 1] Seteo las casilla que hay alrededor
  (Utilities|Time|SetTimerbyEvent (delegate Custom|Tiles) 0.2)
  (CallFunction|UpdatedUI))

(fn ConstructionScript)

(fn TilesatRange
  (bind _outactors (Collision|SphereOverlapActors (Transformation|GetActorLocation) (* (Variables|TilesatRange|GetRange) 99.5) (Utilities|Array|MakeArray "ObjectTypeQuery7") "Bp_Terrain_C" (Utilities|Array|MakeArray self)))
  (Variables|TilesAtRange|SetTilesNearby _outactors))

(fn CheckTokeninTerrain
  (bind _asbp_master_unit (Utilities|Casting|CastToBp_MasterUnit (Utilities|Array|Get(acopy) (Collision|GetOverlappingActors (Variables|Default|GetBox) "/Game/Blueprint/Bp_MasterUnit.Bp_MasterUnit_C" :!class /Script/Engine.PrimitiveComponent))))
  (if (CallFunction|EqualsZero(Int) (Variables|Owner|GetPoints))
    (Variables|Owner|SetTeam? (Variables|/Game/Blueprint/Bp_MasterUnit.Bp_MasterUnit_C|GetTeam _asbp_master_unit))
    (Variables|Owner|SetPoints (CallFunction|PlusOne(Int)))
    (if (== (Variables|Owner|GetTeam?) (Variables|Default|GetUser_Team))
      (Rendering|Material|SetMaterial (Variables|Default|GetStaticMesh) 0 "/Game/Assets/Materials/M_PlayerTerrain.M_PlayerTerrain")
      (CallFunction|UpdatedUI)
      (elif (== (Variables|Owner|GetTeam?) (Variables|Default|GetIA_Team))
        (Rendering|Material|SetMaterial (Variables|Default|GetStaticMesh) 0 "/Game/Assets/Materials/m_EnemyTerrain.m_EnemyTerrain")
        (CallFunction|UpdatedUI)))
    (elif (== (Variables|/Game/Blueprint/Bp_MasterUnit.Bp_MasterUnit_C|GetTeam _asbp_master_unit) (Variables|Owner|GetTeam?))
      (CallFunction|PointstoTeam 1)
      (CallFunction|UpdatedUI)
      (else
        (CallFunction|PointsMInusTeam 1)
        (CallFunction|UpdatedUI)))))

(fn Surrounded
  (Variables|TilesatRange|SetControllerTeams 0)
  (for _array_element (Variables|TilesAtRange|GetTilesNearby)
    (bind _asbp_terrain (Utilities|Casting|CastToBp_Terrain _array_element))
    (if (== (Variables|Bp_Terrain_C|GetTeam? _asbp_terrain) (Variables|Default|GetUser_Team))
      (Variables|TilesatRange|SetControllerTeams (CallFunction|PlusOne(Int) (Variables|TilesatRange|GetControllerTeams)))))
  (if (CallFunction|EqualsNotZero(Int) (Variables|TilesatRange|GetControllerTeams))
    (if (== (CallFunction|MinusOne(Int) (Variables|TilesatRange|GetControllerTeams)) (Utilities|Array|LastIndex (Variables|TilesAtRange|GetTilesNearby)))
      (if (== (Variables|Owner|GetTeam?) (Variables|Default|GetIA_Team))
        (CallFunction|PointsMInusTeam 1)
        (CallFunction|UpdatedUI)
        (elif (CallFunction|EqualsZero(Int) (Variables|Owner|GetTeam?))
          (Variables|Owner|SetTeam? (Variables|Default|GetUser_Team))
          (CallFunction|PointstoTeam 1)
          (Rendering|Material|SetMaterial (Variables|Default|GetStaticMesh) 0 "/Game/Assets/Materials/M_PlayerTerrain.M_PlayerTerrain")
          (CallFunction|UpdatedUI)
          (elif (== (Variables|Owner|GetTeam?) (Variables|Default|GetUser_Team))
            (CallFunction|PointstoTeam 1)
            (CallFunction|UpdatedUI)))))))

(fn UpdatedUI
  (bind _asui_terrain (Utilities|Casting|CastToUI_Terrain (UserInterface|GetUserWidgetObject (Variables|Default|GetWidget))))
  (Rendering|Components|TextRender|SetText (Variables|/Game/Blueprint/UI_Terrain.UI_Terrain_C|Getpoints _asui_terrain) (Utilities|Text|ToText(Integer) (Variables|Owner|GetPoints))))

(fn PointstoTeam
  (params (Points :type Integer))
  (Variables|Owner|SetPoints (+ (Variables|Owner|GetPoints) Points)))

(fn PointsMInusTeam
  (params (Points :type Integer))
  (bind _output_get (Variables|Owner|SetPoints (- (Variables|Owner|GetPoints) Points)))
  (if (CallFunction|EqualsZero(Int) _output_get)
    (Rendering|Material|SetMaterial (Variables|Default|GetStaticMesh) 0 "/Game/Assets/Materials/m_BaseMaterial.m_BaseMaterial")
    (Variables|Owner|SetTeam? 0)))

(fn Spread
  (if (CallFunction|EqualsNotZero(Int) (Variables|Owner|GetPoints))
    (if (>= (Variables|Owner|GetPoints) 10)
      (if (== (Variables|Owner|GetTeam?) (Variables|Default|GetIA_Team))
        (for _array_element (Variables|TilesAtRange|GetTilesNearby)
          (bind _asbp_terrain (Utilities|Casting|CastToBp_Terrain _array_element))
          (if (== (Variables|Default|GetIA_Team) (Variables|Bp_Terrain_C|GetTeam? _asbp_terrain))
            (CallFunction|PointstoTeam _asbp_terrain 1)
            (CallFunction|UpdatedUI _asbp_terrain)
            (elif (== (Variables|Bp_Terrain_C|GetTeam? _asbp_terrain) (Variables|Default|GetUser_Team))
              (CallFunction|PointsMInusTeam _asbp_terrain 1)
              (CallFunction|UpdatedUI _asbp_terrain)
              (elif (== (Variables|Bp_Terrain_C|GetTeam? _asbp_terrain) 0)
                (Variables|Bp_Terrain_C|SetTeam? _asbp_terrain (Variables|Default|GetIA_Team))
                (CallFunction|PointstoTeam _asbp_terrain 1)
                (Rendering|Material|SetMaterial (Variables|Bp_Terrain_C|GetStaticMesh _asbp_terrain) 0 "/Game/Assets/Materials/m_EnemyTerrain.m_EnemyTerrain")
                (CallFunction|UpdatedUI _asbp_terrain)))))))))