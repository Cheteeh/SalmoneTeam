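; MasterDrop_BP is a drop, apparently a base class, that flies to the player and delivers Experience on pickup.
; The construction script loads its ItemData from ItemDrop_DT by row name.
; MagnetMode latches once, stores the player and starts the magnet event, which disables sphere collision.
; A timeline lerps the sphere toward the player's updated position, calling DropInteractMessage and destroying the actor when close or finished.
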(event Custom|Magnet_Event
  (Collision|SetCollisionEnabled (Variables|Default|GetCollisionSphere) "NoCollision")
  (if (Variables|Default|GetMagnetOn?)
    (Variables|Default|SetPlayerPosition (Transformation|GetWorldLocation (Variables|/Script/Engine.Actor|GetRootComponent (Variables|Default|GetPlayer%20Reference))))
    (bind _alpha (Timeline|MoveToTarget PlayFromStart)
      (:Update
        (Variables|Default|SetPlayerPosition (Transformation|GetWorldLocation (Variables|/Script/Engine.Actor|GetRootComponent (Variables|Default|GetPlayer%20Reference))))
        (Transformation|SetWorldLocation (Variables|Default|GetCollisionSphere) (Math|Vector|Lerp(Vector) (Transformation|GetActorLocation) (Variables|Default|GetPlayerPosition) _alpha) false false)
        (if (< (Math|Vector|Distance(Vector) (Transformation|GetActorLocation) (Variables|Default|GetPlayerPosition)) 25.0)
          (Class|VampireInteraction|DropInteract(Message) (Variables|Default|GetPlayer%20Reference) (Variables|Default|GetExperience))
          (Actor|DestroyActor)))
      (:Finished
        (Class|VampireInteraction|DropInteract(Message) (Variables|Default|GetPlayer%20Reference) (Variables|Default|GetExperience))
        (Actor|DestroyActor)))))

(fn ConstructionScript
  (bind _returnvalue (Utilities|GetDataTableRow "/Game/Blueprint/Drops/ItemDrop_DT.ItemDrop_DT" (Variables|Default|GetName))
    (:then
      (Variables|Default|SetItemData _returnvalue))))

(fn DamageInterface
  (params (Damage :type Float%20%28double-precision%29)))

(fn DamagetoPlayer
  (params (DamageToPlayer :type Float%20%28double-precision%29)))

(fn MagnetMode
  (params (PlayerReference :type Player%20Unit%20Object%20Reference))
  (if (not (Variables|Default|GetMagnetOn?))
    (Variables|Default|SetMagnetOn? true)
    (Variables|Default|SetPlayer%20Reference PlayerReference)
    (CallFunction|MagnetEvent)
    (return)))