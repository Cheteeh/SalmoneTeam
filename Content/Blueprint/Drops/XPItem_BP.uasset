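; XPItem_BP is an experience drop pickup that grants XP to the player.
; Its MagnetMode event adds the item data's value to the player's level system and then destroys the drop.
; The construction script runs the parent's script, then swaps the drop mesh material for drops with a specific XP value to distinguish them visually.
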(event EventBeginPlay)

(event Collision|EventActorBeginOverlap
  (params (OtherActor :type Actor%20Object%20Reference)))

(event EventTick
  (params (DeltaSeconds :type Float%20%28single-precision%29)))

(event EventMagnetMode
  (params (PlayerReference :type Player%20Unit%20Object%20Reference))
  (Default|AddXP (Variables|/Game/Blueprint/Player/PlayerUnit.PlayerUnit_C|GetLvlSystem PlayerReference) (Utilities|Struct|BreakItemDrop_ST (Variables|Default|GetItemData)))
  (Actor|DestroyActor))

(fn ConstructionScript
  (|CallParentFunction)
  (if (== (Utilities|Struct|BreakItemDrop_ST (Variables|Default|GetItemData)) 5.0)
    (Rendering|Material|SetMaterial (Variables|Default|GetDropTest) 0 "/Game/Assets/Materials/5XPDrop_MAT.5XPDrop_MAT")))