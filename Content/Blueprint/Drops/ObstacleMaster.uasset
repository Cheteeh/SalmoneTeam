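; ObstacleMaster is a damageable obstacle actor, apparently a base class, that produces drops when destroyed.
; On BeginPlay it hands its own stats to HpSystem and the player's stats to DropSystem.
; DamageInterface applies damage through HpSystem and spawns floating damage text above the actor, red on the killing hit.
; On death DropSystem runs the obstacle drop before the actor destroys itself, while DamageToPlayer simply returns false.
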(event EventBeginPlay
  (Variables|/Game/Blueprint/HpSystem/Hp_System.Hp_System_C|SetStatsComponent (Variables|Default|GetHp_System) (Variables|Default|GetStatsComponent))
  (Variables|/Game/Blueprint/Drops/DropSystem.DropSystem_C|SetStatsComponent (Variables|Default|GetDropSystem) (Variables|Default|GetPlayerStatsComponent)))

(fn ConstructionScript)

(fn Dead
  (Default|ObstacleDrop (Variables|Default|GetDropSystem))
  (Actor|DestroyActor))

(fn DamageInterface
  (params (Damage :type Float%20%28double-precision%29))
  (bind _returnvalue (Transformation|GetActorLocation))
  (bind _returnvalue_2 (Transformation|GetActorLocation))
  (bind _dead_ (Default|ApplyDamage (Variables|Default|GetHp_System) Damage))
  (if _dead_
    (Game|SpawnActorfromClass "/Game/Blueprint/Interfaz/Bp_FloatingText.Bp_FloatingText_C" (Math|Transform|MakeTransform (Math|Vector|MakeVector (.x _returnvalue_2) (.y _returnvalue_2) (+ (.z _returnvalue_2) 4e+01)) "0, 0, 0" "1.000000,1.000000,1.000000") "AlwaysSpawn" 0 Damage (Math|Color|MakeColor 0 0 255) 0)
    (CallFunction|Dead)
    (else
      (Game|SpawnActorfromClass "/Game/Blueprint/Interfaz/Bp_FloatingText.Bp_FloatingText_C" (Math|Transform|MakeTransform (Math|Vector|MakeVector (.x _returnvalue) (.y _returnvalue) (+ (.z _returnvalue) 4e+01)) "0, 0, 0" "1.000000,1.000000,1.000000") "AlwaysSpawn" 0 Damage "(B=0,G=0,R=0,A=0)" 0)))
  (return true))

(fn DamagetoPlayer
  (params (DamageToPlayer :type Float%20%28double-precision%29))
  (return false))