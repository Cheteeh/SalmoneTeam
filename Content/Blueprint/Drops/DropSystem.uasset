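; Drop system that spawns XP or chest pickups at a given location through its EnemyDrop function.
; A random roll against drop chance plus the stats component's Luck gates every drop, bosses included.
; Bosses then make a second Luck-boosted roll for a chest, falling back to a five-XP drop, while other enemies drop five or one XP based on their XP value.
; ObstacleDrop is an empty stub.
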(event EventBeginPlay)

(fn EnemyDrop
  (params (Boss :type Boolean) (Location :type Vector) (XPValue :type Integer))
  (bind _drop (CallFunction|CalcDropChanceEnemy))
  (if _drop
    (if Boss
      (bind _drop_2 (CallFunction|CalcBossChestProb))
      (if _drop_2
        (Game|SpawnActorfromClass "/Game/Blueprint/Drops/1ChestDrop_BP.1ChestDrop_BP_C" (Math|Transform|MakeTransform Location "0, 0, 0" "1.000000,1.000000,1.000000") "Undefined" 0 0)
        (else
          (Game|SpawnActorfromClass "/Game/Blueprint/Drops/5XPDrop_BP.5XPDrop_BP_C" (Math|Transform|MakeTransform Location "0, 0, 0" "1.000000,1.000000,1.000000") "Undefined" 0 0)))
      (elif (== XPValue 5)
        (Game|SpawnActorfromClass "/Game/Blueprint/Drops/5XPDrop_BP.5XPDrop_BP_C" (Math|Transform|MakeTransform Location "0, 0, 0" "1.000000,1.000000,1.000000") "Undefined" 0 0)
        (else
          (Game|SpawnActorfromClass "/Game/Blueprint/Drops/1XPDrop_BP.1XPDrop_BP_C" (Math|Transform|MakeTransform Location "0, 0, 0" "1.000000,1.000000,1.000000") "Undefined" 0 0))))))

(fn CalcDropChanceEnemy
  (if (< (Math|Random|RandomFloatinRange 0.0 1e+02) (+ (Variables|Default|GetDropChance) (Utilities|Struct|BreakPlayerStructure (Variables|/Game/Blueprint/StatComponent/StatsComponent.StatsComponent_C|GetStructure (Variables|Default|GetStatsComponent)))))
    (return true)
    (else
      (return false))))

(fn CalcBossChestProb
  (if (< (Math|Random|RandomFloatinRange 0.0 1e+02) (+ (Variables|Default|GetDropChanceChest) (Utilities|Struct|BreakPlayerStructure (Variables|/Game/Blueprint/StatComponent/StatsComponent.StatsComponent_C|GetStructure (Variables|Default|GetStatsComponent)))))
    (return true)
    (else
      (return false))))

(fn ObstacleDrop)