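; MainGameInstance is the game instance that holds the selected character and starts gameplay with it.
; SetupCharacter stores the selection in CharacterSelected.
; StartGameplay spawns a PlayerUnit, copies the selection's CharacterStats into its StatsComponent, possesses it with the first player controller, then calls InitializeCharacter.
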(fn StartGameplay
  (bind _returnvalue (Game|SpawnActorfromClass "/Game/Blueprint/Player/PlayerUnit.PlayerUnit_C" (Math|Transform|MakeTransform "0, 0, 0" "0, 0, 0" "1.000000,1.000000,1.000000") "Undefined" 0 (Game|Player|GetPlayerPawn 0)))
  (Variables|/Game/Blueprint/StatComponent/StatsComponent.StatsComponent_C|SetStructure (Variables|/Game/Blueprint/Player/PlayerUnit.PlayerUnit_C|GetStatsComponent _returnvalue) (Utilities|Struct|BreakUI_CharacterStructure (Variables|Default|GetCharacterSelected)))
  (Pawn|Possess (Game|GetPlayerController 0) _returnvalue)
  (Default|InitializeCharacter _returnvalue))

(fn SetupCharacter
  (params (CharacterSelected :type UI%20Character%20Structure%20Structure))
  (Variables|Default|SetCharacterSelected CharacterSelected))