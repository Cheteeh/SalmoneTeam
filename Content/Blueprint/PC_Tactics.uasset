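; Player controller for a tactics game that lets the mouse drag units between grid tiles and attack by dropping.
; Pressing picks a unit and records its origin tile; Tick moves it along the terrain under the cursor with a height offset, using separate object-type traces.
; Releasing on a free tile snaps to its "Centro" socket and transfers occupancy.
; An occupied tile returns the unit and applies its Damage to the occupant.
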(event EventTick
  (params (DeltaSeconds :type Float%20%28single-precision%29))
  (bind _array (Utilities|Array|MakeArray "ObjectTypeQuery7"))
  (bind (_hitresult _returnvalue) (Class|PlayerController|GetHitResultUnderCursorforObjects _array true))
  (bind _location (Collision|BreakHitResult _hitresult))
  (if (Variables|Default|GetGrab?)
    (Variables|Default|GetGrabbedComponent
      (:then
        (if _returnvalue
          (Transformation|SetWorldLocation (Variables|Default|GetGrabbedComponent) (Math|Vector|MakeVector (.x _location) (.y _location) (+ (.z _location) (Variables|Default|GetFeedbackGrab))) false false)))
      (:else))))

(event Input|MouseEvents|LeftMouseButton
  (params (Key :type Key%20Structure :default "None"))
  (:Pressed
    (CallFunction|HoldUnit))
  (:Released
    (if (Variables|Default|GetGrab?)
      (CallFunction|DropUnit))))

(fn ConstructionScript)

(fn DropUnit
  (bind _array (Utilities|Array|MakeArray "ObjectTypeQuery7"))
  (bind _ref_grid_ (Variables|Default|GetRef_Grid?))
  (bind _hitresult (Class|PlayerController|GetHitResultUnderCursorforObjects _array true))
  (bind (_bblockinghit _binitialoverlap _time _distance _location _impactpoint _normal _impactnormal _physmat _hitactor) (Collision|BreakHitResult _hitresult))
  (if _bblockinghit
    (bind _asbp_terrain (Utilities|Casting|CastToBp_Terrain _hitactor))
    (if (Variables|/Game/Blueprint/Grid/Bp_Terrain.Bp_Terrain_C|GetEstaOcupada? _asbp_terrain)
      (Transformation|SetWorldLocation (Variables|Default|GetGrabbedComponent) (Variables|Default|GetPosicionInicial) false false :!label _label)
      (bind _asbp_terrain_2 (Utilities|Casting|CastToBp_Terrain (.HitActor (Collision|BreakHitResult (.HitResult (Class|PlayerController|GetHitResultUnderCursorforObjects (Utilities|Array|MakeArray "ObjectTypeQuery7") true))))))
      (bind _asbp_master_unit (Utilities|Casting|CastToBp_MasterUnit (Components|GetOwner (Variables|/Game/Blueprint/Grid/Bp_Terrain.Bp_Terrain_C|GetQuienMeocupa _asbp_terrain_2))))
      (bind _asbp_master_unit_2 (Utilities|Casting|CastToBp_MasterUnit (Components|GetOwner (Variables|Default|GetGrabbedComponent))))
      (Default|ApplyDamage _asbp_master_unit (Variables|/Game/Blueprint/Unit/Bp_MasterUnit.Bp_MasterUnit_C|GetDamage _asbp_master_unit_2))
      (else
        (Transformation|SetWorldLocation (Variables|Default|GetGrabbedComponent) (Transformation|GetSocketLocation (Variables|/Game/Blueprint/Grid/Bp_Terrain.Bp_Terrain_C|GetStaticMesh _asbp_terrain) "Centro") false false)
        (Variables|/Game/Blueprint/Grid/Bp_Terrain.Bp_Terrain_C|SetEstaOcupada? _asbp_terrain true)
        (Variables|/Game/Blueprint/Grid/Bp_Terrain.Bp_Terrain_C|SetQuienMeocupa _asbp_terrain (Variables|Default|GetGrabbedComponent))
        (Variables|/Game/Blueprint/Grid/Bp_Terrain.Bp_Terrain_C|SetEstaOcupada? _ref_grid_ false)
        (Variables|/Game/Blueprint/Grid/Bp_Terrain.Bp_Terrain_C|SetQuienMeocupa _ref_grid_ 0)))
    (else
      (goto _label)))
  (Variables|Default|SetGrab? false))

(fn HoldUnit
  (bind _array (Utilities|Array|MakeArray "ObjectTypeQuery8"))
  (bind (_hitresult _returnvalue) (Class|PlayerController|GetHitResultUnderCursorforObjects _array true))
  (if _returnvalue
    (Variables|Default|SetGrab? true)
    (Variables|Default|SetGrabbedComponent (.HitComponent (Collision|BreakHitResult _hitresult)))
    (Variables|Default|SetPosicionInicial (Transformation|GetWorldLocation (Variables|Default|GetGrabbedComponent)))
    (bind _asbp_terrain (Utilities|Casting|CastToBp_Terrain (.HitActor (Collision|BreakHitResult (.HitResult (Class|PlayerController|GetHitResultUnderCursorforObjects (Utilities|Array|MakeArray "ObjectTypeQuery7") true))))))
    (Variables|Default|SetRef_Grid? _asbp_terrain)
    (else
      (return))))