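; Enemy unit that loads stats from a data table and chases its Target with AIMoveTo.
; Sphere overlap starts a looping timer damaging the player through an interface; overlap end nulls the target but only unpauses the timer.
; Incoming damage goes through HpSystem and spawns floating text, red on lethal hits.
; Death records the kill, triggers DropSystem's XP drop, decrements SpawnSystem's live count and destroys the actor.
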(event OnComponentBeginOverlap(Sphere)
  (params (OverlappedComponent :type Primitive%20Component%20Object%20Reference) (OtherActor :type Actor%20Object%20Reference) (OtherComp :type Primitive%20Component%20Object%20Reference) (OtherBodyIndex :type Integer) (bFromSweep :type Boolean) (SweepResult :type Hit%20Result%20Structure%20%28by%20ref%29))
  (if (== (Utilities|GetClass OtherActor) "/Game/Blueprint/Player/PlayerUnit.PlayerUnit_C")
    (if (Utilities|DoesObjectImplementInterface OtherActor "/Game/Blueprint/Vampire_Interaction.Vampire_Interaction_C")
      (Variables|Default|SetActorToDamage OtherActor)
      (bind _returnvalue (Utilities|Time|SetTimerbyEvent (delegate Custom|CustomEvent_0) 0.25 true))
      (Variables|Default|SetTimerToDamage _returnvalue))))

(event OnComponentEndOverlap(Sphere)
  (params (OverlappedComponent :type Primitive%20Component%20Object%20Reference) (OtherActor :type Actor%20Object%20Reference) (OtherComp :type Primitive%20Component%20Object%20Reference) (OtherBodyIndex :type Integer))
  (if (== (Utilities|GetClass OtherActor) "/Game/Blueprint/Player/PlayerUnit.PlayerUnit_C")
    (if (Utilities|DoesObjectImplementInterface OtherActor "/Game/Blueprint/Vampire_Interaction.Vampire_Interaction_C")
      (Variables|Default|SetActorToDamage 0)
      (Utilities|Time|UnpauseTimerbyHandle (Variables|Default|GetTimerToDamage)))))

(event Custom|CustomEvent_0
  (Class|VampireInteraction|DamagetoPlayer(Message) (Variables|Default|GetActorToDamage) (Variables|Default|GetDamageDealt_0)))

(event EventBeginPlay
  (bind _enemystructure (Variables|Default|GetEnemyStructure))
  ;[1 1 1] Seteo de Valores e inicio de la IA sencilla para perseguir al player
  (bind _returnvalue (Utilities|GetDataTableRow (.datatable _enemystructure) (.rowname _enemystructure))
    (:then
      (Utilities|Struct|SetmembersinHp_Structure (.HpStructure (Utilities|Struct|BreakPlayerStructure (Variables|/Game/Blueprint/StatComponent/StatsComponent.StatsComponent_C|GetStructure (Variables|Default|GetStatsComponent)))) (.Hp (Utilities|Struct|BreakEnemyStructure _returnvalue)))
      (Variables|Default|SetDamageDealt_0 (.Damage (Utilities|Struct|BreakEnemyStructure _returnvalue)))
      (Variables|Default|SetSpeed (.Speed (Utilities|Struct|BreakEnemyStructure _returnvalue)))
      (AI|AIMoveTo (AI|GetAIController (Pawn|GetController)) "0, 0, 0" (Variables|Default|GetTarget) 0.0 "Disable" "Disable" false true true "Disable"))))

(fn ConstructionScript
  (Variables|/Game/Blueprint/HpSystem/Hp_System.Hp_System_C|SetStatsComponent (Variables|Default|GetHp_System) (Variables|Default|GetStatsComponent))
  (Variables|/Game/Blueprint/Drops/DropSystem.DropSystem_C|SetPlayerStatsComponent (Variables|Default|GetDropSystem) (Variables|Default|GetPlayerStatsComponent)))

(fn Dead
  (bind _dt_enemystructure (Variables|Default|GetDT_EnemyStructure))
  (Default|AddEnemyDeath (Variables|Default|GetPlayerStatsComponent))
  ;[1 1 1] *** Añadir logica para el drop de XP
  (Default|EnemyDrop (Variables|Default|GetDropSystem) (.boss _dt_enemystructure) (Transformation|GetActorLocation) (.xpvalue _dt_enemystructure))
  ;[0 0 0 1 10] Eliminamos el enemigo del controlador
  (Math|Integer|DecrementInt (Variables|/Game/Blueprint/Spawner/SpawnerComponent.SpawnerComponent_C|GetEnemyAmountInPlay (Variables|Default|GetSpawnSystem))
    (:%20%20
      (Actor|DestroyActor))))

(fn DamageInterface
  (params (Damage :type Float%20%28double-precision%29))
  (bind _returnvalue (Transformation|GetActorLocation))
  (bind _returnvalue_2 (Transformation|GetActorLocation))
  ;[1 1 1] Applicamos el daño del jugador al enemigo
  (bind _dead_ (Default|ApplyDamage (Variables|Default|GetHp_System) Damage))
  ;[1 1 1] Añadimos el floating Damage Text
  (if _dead_
    (Game|SpawnActorfromClass "/Game/Blueprint/Interfaz/Bp_FloatingText.Bp_FloatingText_C" (Math|Transform|MakeTransform (Math|Vector|MakeVector (.x _returnvalue) (.y _returnvalue) (+ (.z _returnvalue) 4e+01)) "0, 0, 0" "1.000000,1.000000,1.000000") "AlwaysSpawn" 0 Damage (Math|Color|MakeColor 0 0 255) 0)
    ;[1 1 1] Destruimos la unidad
    (CallFunction|Dead)
    (else
      (Game|SpawnActorfromClass "/Game/Blueprint/Interfaz/Bp_FloatingText.Bp_FloatingText_C" (Math|Transform|MakeTransform (Math|Vector|MakeVector (.x _returnvalue_2) (.y _returnvalue_2) (+ (.z _returnvalue_2) 4e+01)) "0, 0, 0" "1.000000,1.000000,1.000000") "AlwaysSpawn" 0 Damage "(B=0,G=0,R=0,A=0)" 0)))
  (return true))

(fn DamagetoPlayer
  (params (DamageToPlayer :type Float%20%28double-precision%29))
  ;[1 1 1] Pasamos el daño que causa al player el enemigo
)

(fn MagnetMode
  (params (PlayerReference :type Actor%20Object%20Reference))
  ;[1 1 1] No se usa
)