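; Base weapon actor that auto-fires projectiles on a looping timer, with stats loaded by level from a data table.
; Calc functions apply StatsComponent percentage modifiers to damage, duration, projectile speed and fire interval, which is clamped to a minimum.
; Each shot spawns the row's projectile at the actor's transform with those values.
; UpdateWeapon swaps rows and calls Update, which recalculates stats, pauses the old timer and starts another.
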(event Custom|FireWeapon
  (Game|SpawnActorfromClass (.Projectile (Utilities|Struct|BreakWeaponStructure (Variables|Data|GetStructure))) (Math|Transform|MakeTransform (Transformation|GetActorLocation) (Transformation|GetActorRotation) "1.000000,1.000000,1.000000") "Undefined" 0 (Variables|Controllers|GetDamage_Calc) (Variables|Controllers|GetDuration_Calc) (Variables|Controllers|GetProjectionSpeed_Calc) 0))

(event Custom|Update
  (CallFunction|RateOfFireCalc)
  (CallFunction|DamageCalc)
  (CallFunction|DurationCalc)
  (CallFunction|ProjectileSpeedCalc)
  (Utilities|Time|PauseTimerbyHandle (Variables|Controllers|GetTimerController))
  (bind _returnvalue (Utilities|Time|SetTimerbyEvent (EventDispatchers|CreateEvent :!event Custom|FireWeapon) (Variables|Controllers|GetRateOfFIre_Calc) true))
  (Variables|Controllers|SetTimerController _returnvalue))

(event EventBeginPlay
  (bind _returnvalue (Utilities|GetDataTableRow (Variables|Data|GetSpawnData) (Variables|Data|GetSpawnLevel))
    (:then
      (Variables|Data|SetStructure _returnvalue)
      (CallFunction|RateOfFireCalc)
      (CallFunction|DamageCalc)
      (CallFunction|DurationCalc)
      (CallFunction|ProjectileSpeedCalc)
      (bind _returnvalue_2 (Utilities|Time|SetTimerbyEvent (EventDispatchers|CreateEvent :!event Custom|FireWeapon) (Variables|Controllers|GetRateOfFIre_Calc) true))
      (Variables|Controllers|SetTimerController _returnvalue_2)
      (EventDispatchers|BindEventtoCallUptade (Variables|Default|GetStatsComponent) (EventDispatchers|CreateEvent :!event Custom|Update)))
    (:RowNotFound
      (Development|PrintString "Arma No encontrtada")
      (Actor|DestroyActor))))

(fn ConstructionScript)

(fn RateOfFireCalc
  (bind _structure (Variables|Data|GetStructure))
  (bind _statscomponent (Variables|Default|GetStatsComponent))
  (bind _rateoffire (Utilities|Struct|BreakWeaponStructure _structure))
  (bind _structure_2 (Variables|/Game/Blueprint/StatComponent/StatsComponent.StatsComponent_C|GetStructure _statscomponent))
  (bind _rateoffiremultiplier (Utilities|Struct|BreakPlayerStructure _structure_2))
  (bind _returnvalue (* _rateoffiremultiplier _rateoffire))
  (bind _returnvalue_2 (/ _returnvalue 1e+02))
  (bind _returnvalue_3 (- _rateoffire _returnvalue_2))
  (Variables|Controllers|SetRateOfFIre_Calc (Math|Float|SelectFloat 0.001 _returnvalue_3 (< _returnvalue_3 0.001)))
  (return))

(fn DamageCalc
  (bind _structure (Variables|Data|GetStructure))
  (bind _damage (Utilities|Struct|BreakWeaponStructure _structure))
  (Variables|Controllers|SetDamage_Calc (+ _damage (/ (* (Utilities|Struct|BreakPlayerStructure (Variables|/Game/Blueprint/StatComponent/StatsComponent.StatsComponent_C|GetStructure (Variables|Default|GetStatsComponent))) _damage) 1e+02)))
  (return))

(fn DurationCalc
  (bind _structure (Variables|Data|GetStructure))
  (bind _duration (Utilities|Struct|BreakWeaponStructure _structure))
  (Variables|Controllers|SetDuration_Calc (+ _duration (/ (* (Utilities|Struct|BreakPlayerStructure (Variables|/Game/Blueprint/StatComponent/StatsComponent.StatsComponent_C|GetStructure (Variables|Default|GetStatsComponent))) _duration) 1e+02)))
  (return))

(fn ProjectileSpeedCalc
  (bind _structure (Variables|Data|GetStructure))
  (bind _projectilespeed (Utilities|Struct|BreakWeaponStructure _structure))
  (Variables|Controllers|SetProjectionSpeed_Calc (+ _projectilespeed (/ (* (Utilities|Struct|BreakPlayerStructure (Variables|/Game/Blueprint/StatComponent/StatsComponent.StatsComponent_C|GetStructure (Variables|Default|GetStatsComponent))) _projectilespeed) 1e+02)))
  (return))

(fn UpdateWeapon
  (params (Level :type Name))
  (bind _returnvalue (Utilities|GetDataTableRow (Variables|Data|GetSpawnData) Level)
    (:then
      (Variables|Data|SetStructure _returnvalue)
      (CallFunction|Update)
      (return true))
    (:RowNotFound
      (Development|PrintString "Arma no encontrada")
      (return false))))