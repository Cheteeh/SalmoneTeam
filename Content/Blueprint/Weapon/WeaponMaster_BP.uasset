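; Base weapon actor that automatically fires by spawning its projectile class at its own transform on a looping timer set at BeginPlay.
; Construction loads its stats by row name from Weapon_DT.
; UpgradeWeapon looks up a name-plus-level row in WeaponUpgrades_DT and applies its first effect to level, fire interval or projectile count.
; The running timer is not reset on upgrade, and firing ignores projectile count.
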(event Custom|FireWeapon
  (Game|SpawnActorfromClass (.Projectile (Utilities|Struct|BreakWeapon_ST (Variables|Default|GetData))) (Transformation|GetActorTransform) "Undefined" 0 0))

(event EventBeginPlay
  (Utilities|Time|SetTimerbyEvent (delegate Custom|FireWeapon) (Utilities|Struct|BreakWeapon_ST (Variables|Default|GetData)) true))

(fn ConstructionScript
  (CallFunction|Initialize))

(fn UpgradeWeapon
  (bind _data (Variables|Default|GetData))
  (bind _data_2 (Variables|Default|GetData))
  (bind _data_3 (Variables|Default|GetData))
  (bind _data_4 (Variables|Default|GetData))
  (bind (_level _maxlevel) (Utilities|Struct|BreakWeapon_ST _data))
  (bind (_name _level_2) (Utilities|Struct|BreakWeapon_ST _data_4))
  (bind _returnvalue (Utilities|GetDataTableRow "/Game/Blueprint/Weapon/WeaponUpgrades_DT.WeaponUpgrades_DT" (Utilities|String|StringToName (Utilities|String|Append (Utilities|String|ToString(Name) _name) (Utilities|String|ToString(Integer) _level_2))))
    (:then
      (LocalVariables|SetAm (.effect1_amount _returnvalue))
      (switch name (.effect1_name _returnvalue)
        (:Default
          (Development|PrintString "Upgrade weapon failed for some reason!!!" true true "(R=1.000000,G=0.000000,B=0.070897,A=1.000000)" 5.0))
        (:Level
          (if (<= (+ _level (Math|Float|Truncate (LocalVariables|GetAm))) _maxlevel)
            (Utilities|Struct|SetmembersinWeapon_ST (Variables|Default|GetData) (+ _level (Math|Float|Truncate (LocalVariables|GetAm))))
            (else
              (Utilities|Struct|SetmembersinWeapon_ST (Variables|Default|GetData) false))))
        (:RateOfFire
          (Utilities|Struct|SetmembersinWeapon_ST _data_2 (+ (Utilities|Struct|BreakWeapon_ST _data_2) (LocalVariables|GetAm))))
        (:NumberOfProjectiles
          (Utilities|Struct|SetmembersinWeapon_ST _data_3 (+ (Utilities|Struct|BreakWeapon_ST _data_3) (Math|Float|Truncate (LocalVariables|GetAm)))))))))

(fn Initialize
  (bind _returnvalue (Utilities|GetDataTableRow "/Game/Blueprint/Weapon/Weapon_DT.Weapon_DT" (Variables|Default|GetName))
    (:then
      (Variables|Default|SetData _returnvalue))
    (:RowNotFound
      (Development|PrintString "WEAPON INIT FAILED" true true "(R=1.000000,G=0.000000,B=0.038562,A=1.000000)"))))