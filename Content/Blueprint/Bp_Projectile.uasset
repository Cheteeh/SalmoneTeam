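; Projectile actor that creeps toward a Destination point on the X and Y axes, with no sweep or hit handling.
; Each Tick, until its location matches Destination, it adds a local offset of one X unit toward the target, with Y scaled by the remaining slope.
; The step ignores delta time, so speed depends on frame rate and slope, and Z never changes.
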(event EventTick
  (params (DeltaSeconds :type Float%20%28single-precision%29))
  (bind _returnvalue (Transformation|GetActorLocation))
  (bind _destination (Variables|Default|GetDestination))
  (bind _returnvalue_2 (- _returnvalue _destination))
  (bind (_x _y) (Math|Vector|BreakVector _returnvalue_2))
  (if (not (Math|Vector|Equal(Vector) _returnvalue (Variables|Default|GetDestination) 0.0001))
    (Transformation|AddActorLocalOffset (Math|Vector|MakeVector (Math|Conversions|ToFloat(Integer) (Math|Integer|SelectInt -1 1 (CallFunction|BiggerThanZero(Float) _x))) (/ (Math|Conversions|ToFloat(Integer) (Math|Integer|SelectInt -1 1 (CallFunction|BiggerThanZero(Float) _y))) (Math|Float|Absolute(Float) (/ _x _y))) 0.0) false false)))

(fn ConstructionScript)