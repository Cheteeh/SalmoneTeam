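; Hp_System is a health system that handles damage, armor, healing and regeneration through a shared HpStructure.
; ApplyDamage subtracts flat armor from incoming damage, floors CurrentHP at zero, and returns the damage dealt and whether it was lethal.
; Heal caps CurrentHP at HpMax.
; When RecoveryHp is positive, CheckRecovery starts a looping one-second timer whose Recovery function calls Heal while health is below max.
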(fn ApplyDamage
  (params (DamageToDeal :type Float%20%28double-precision%29))
  (bind _damage_output (CallFunction|Armor DamageToDeal))
  (if (<= _damage_output 0.0)
    ;[1 1 1] Añadir Feedback de no DAÑO
    (return false 0.0)
    (else
      ;[1 1 1] Aplicamos el daño
      (if (> (- (Utilities|Struct|BreakHp_Structure (Variables|Default|GetHpStructure)) _damage_output) 0.0)
        (Utilities|Struct|SetmembersinHp_Structure (Variables|Default|GetHpStructure) (- (Utilities|Struct|BreakHp_Structure (Variables|Default|GetHpStructure)) _damage_output))
        (return false _damage_output)
        (else
          ;[1 1 1] Si ha muerto se devuelte True
          (Utilities|Struct|SetmembersinHp_Structure (Variables|Default|GetHpStructure) 0.0)
          (return true _damage_output))))))

(fn Heal
  (params (HpToHeal :type Float%20%28double-precision%29))
  (bind _hpstructure (Variables|Default|GetHpStructure))
  (bind _hpstructure_2 (Variables|Default|GetHpStructure))
  (bind (_hpmax _currenthp) (Utilities|Struct|BreakHp_Structure _hpstructure))
  (bind _returnvalue (+ HpToHeal _currenthp))
  (if (> _returnvalue _hpmax)
    (Utilities|Struct|SetmembersinHp_Structure _hpstructure_2 (Utilities|Struct|BreakHp_Structure _hpstructure_2))
    (else
      (Utilities|Struct|SetmembersinHp_Structure (Variables|Default|GetHpStructure) _returnvalue))))

(fn CheckRecovery
  (if (> (Utilities|Struct|BreakHp_Structure (Variables|Default|GetHpStructure)) 0.0)
    (bind _returnvalue (Utilities|Time|SetTimerbyFunctionName 0 "Recovery" 1.0 true))
    (Variables|Default|SetRecoveryTimer _returnvalue)))

(fn Recovery
  (bind _hpstructure (Variables|Default|GetHpStructure))
  (bind (_hpmax _currenthp) (Utilities|Struct|BreakHp_Structure _hpstructure))
  (if (< _currenthp _hpmax)
    (CallFunction|Heal (Utilities|Struct|BreakHp_Structure (Variables|Default|GetHpStructure)))))

(fn Armor
  (params (DamageInput :type Float%20%28double-precision%29))
  (bind _hpstructure (Variables|Default|GetHpStructure))
  (bind _armor (Utilities|Struct|BreakHp_Structure _hpstructure))
  (bind _returnvalue (- DamageInput _armor))
  (if (> _armor 0.0)
    (return (Math|Float|SelectFloat 0.0 _returnvalue (<= _returnvalue 0.0)))
    (else
      (return DamageInput))))