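; LvlSystem tracks XP and levels up to a level cap and notifies the HUD.
; AddXP fills a buffer that Tick eases CurrentXP toward with a rounded-up FInterpTo, updating the bar percentage.
; Reaching the max triggers LevelUP, which multiplies the requirement and carries surplus buffered XP over.
; At the cap XP is pinned to the max, so the HUD's LevelUp call repeats every tick.
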(event EventBeginPlay
  ;[1 1 1] Calculamos el porcentaje de la barra
  (CallFunction|CalculatePercentage))

(event EventTick
  (params (DeltaSeconds :type Float%20%28single-precision%29))
  ;[1 1 1] Calculamos de forma progresiva el porcentaje de la barra de vida
  (Variables|Default|SetCurrentXP (Math|Conversions|ToFloat(Integer) (Math|Float|Ceil (Math|Interpolation|FInterpTo (Variables|Default|GetCurrentXP) (Variables|Default|GetBufferXp) DeltaSeconds 5.0))))
  (CallFunction|CalculatePercentage)
  ;[1 1 1] Comprobamos si es necesario un level UP
  (if (>= (Variables|Default|GetCurrentXP) (Variables|Default|GetCurrentMaxXP))
    (CallFunction|LevelUP)
    (Default|LevelUp (Variables|Reference|GetHudRefence))))

(fn CalculatePercentage
  (Variables|Default|SetCurrentPercentage (/ (Variables|Default|GetCurrentXP) (Variables|Default|GetCurrentMaxXP))))

(fn CalculateMaxXP
  (Variables|Default|SetCurrentMaxXP (Math|Conversions|ToFloat(Integer) (Math|Float|Ceil (* (Variables|Default|GetCurrentMaxXP) 1.7)))))

(fn AddXP
  (params (AddedXp :type Float%20%28double-precision%29))
  (Variables|Default|SetBufferXp (+ AddedXp (Variables|Default|GetBufferXp))))

(fn LevelUP
  (bind _currentmaxxp (Variables|Default|GetCurrentMaxXP))
  (if (>= (Variables|Default|GetCurrentLevel) (Variables|Default|GetLevelCap))
    (Variables|Default|SetCurrentXP _currentmaxxp)
    (Variables|Default|SetBufferXp _currentmaxxp)
    (else
      (Math|Integer|IncrementInt (Variables|Default|GetCurrentLevel)
        (:%20%20
          (LocalVariables|SetRemainingXP (- (Variables|Default|GetBufferXp) (Variables|Default|GetCurrentMaxXP)))
          (CallFunction|CalculateMaxXP)
          (Variables|Default|SetCurrentXP 0.0)
          (Variables|Default|SetBufferXp 0.0)
          (CallFunction|AddXP (LocalVariables|GetRemainingXP)))))))