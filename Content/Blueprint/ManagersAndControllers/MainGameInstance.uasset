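; Game instance that manages persistent progression (money, character unlocks and purchases, power-up levels) and spawns the selected character for gameplay.
; Init loads or creates the save, adding missing power-ups from a master data table at level zero; setters save immediately.
; StartGameplay sums each power-up's level-named data table row into PowerUpStats, adds that to the character's stats, then spawns and possesses PlayerUnit with its default weapon.
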(event EventInit
  (bind _returnvalue (SaveGame|DoesSaveGameExist (Variables|Default|GetSaveDataSlot)))
  (if _returnvalue
    (bind _returnvalue_2 (SaveGame|LoadGamefromSlot (Variables|Default|GetSaveDataSlot)))
    (bind _asmain_save_game (Utilities|Casting|CastToMainSaveGame _returnvalue_2))
    (Variables|Default|SetSaveGameData _asmain_save_game)
    (PowerUps|InitPowerUps)
    (else
      (bind _returnvalue_3 (SaveGame|CreateSaveGameObject "/Game/Blueprint/ManagersAndControllers/MainSaveGame.MainSaveGame_C"))
      (Variables|Default|SetSaveGameData _returnvalue_3)
      (PowerUps|InitPowerUps))))

(fn StartGameplay
  (bind _characterselected (Variables|Default|GetCharacterSelected))
  (bind (_defaultweapon _characterstats) (Utilities|Struct|BreakUI_CharacterStructure _characterselected))
  (PowerUps|CalcPowerUpStats)
  (PowerUps|ApplyPowerUps)
  (bind _returnvalue (Game|SpawnActorfromClass "/Game/Blueprint/Actors/PlayerUnit.PlayerUnit_C" (Math|Transform|MakeTransform "0, 0, 0" "0, 0, 0" "1.000000,1.000000,1.000000") "Undefined" 0 (Game|Player|GetPlayerPawn 0)))
  (Variables|/Game/Blueprint/Components/StatsComponent.StatsComponent_C|SetStructure (Variables|/Game/Blueprint/Actors/PlayerUnit.PlayerUnit_C|GetStatsComponent _returnvalue) _characterstats)
  (Pawn|Possess (Game|GetPlayerController 0) _returnvalue)
  (Default|InitializeCharacter _returnvalue)
  (Default|AddWeapon (Variables|/Game/Blueprint/Actors/PlayerUnit.PlayerUnit_C|GetWeaponSystem _returnvalue) _defaultweapon))

(fn SetupCharacter
  (params (CharacterSelected :type UI%20Character%20Structure%20Structure))
  (Variables|Default|SetCharacterSelected CharacterSelected))

(fn SaveGame
  (SaveGame|SaveGametoSlot (Variables|Default|GetSaveGameData) (Variables|Default|GetSaveDataSlot)))

(fn SavePlayerUnlock
  (params (CharacterUnlocks :type Map%20of%20Names%20to%20Booleans))
  (|SetBy-RefVar (Variables|/Game/Blueprint/ManagersAndControllers/MainSaveGame.MainSaveGame_C|GetCharacterUnlock (Variables|Default|GetSaveGameData)) CharacterUnlocks)
  (SaveGame|SaveGame))

(fn LoadPlayerUnlock
  (return (Variables|/Game/Blueprint/ManagersAndControllers/MainSaveGame.MainSaveGame_C|GetCharacterUnlock (Variables|Default|GetSaveGameData))))

(fn SavePlayerBuys
  (params (Value :type Map%20of%20Names%20to%20Booleans))
  (|SetBy-RefVar (Variables|/Game/Blueprint/ManagersAndControllers/MainSaveGame.MainSaveGame_C|GetCharacterBuy (Variables|Default|GetSaveGameData)) Value)
  (SaveGame|SaveGame))

(fn LoadPlayersBuy
  (return (Variables|/Game/Blueprint/ManagersAndControllers/MainSaveGame.MainSaveGame_C|GetCharacterBuy (Variables|Default|GetSaveGameData))))

(fn SaveMoney
  (params (Money :type Integer))
  (Variables|/Game/Blueprint/ManagersAndControllers/MainSaveGame.MainSaveGame_C|SetMoney (Variables|Default|GetSaveGameData) Money)
  (SaveGame|SaveGame))

(fn LoadMoney
  (return (Variables|/Game/Blueprint/ManagersAndControllers/MainSaveGame.MainSaveGame_C|GetMoney (Variables|Default|GetSaveGameData))))

(fn ResetSaveGame
  (SaveGame|DeleteGameinSlot (Variables|Default|GetSaveDataSlot)))

(fn InitPowerUps
  ;[0 0 0] Comprueba si hay PowerUpsNuevos
  (bind _outrownames (DataTable|GetDataTableRowNames "/Game/Blueprint/Data/Datatables/PowerUps/PowerUpsList_DT.PowerUpsList_DT"))
  (if (not (== (Utilities|Array|LastIndex _outrownames) (Utilities|Map|Length (Variables|/Game/Blueprint/ManagersAndControllers/MainSaveGame.MainSaveGame_C|GetPowerUps (Variables|Default|GetSaveGameData)))))
    (bind _outrownames_2 (DataTable|GetDataTableRowNames "/Game/Blueprint/Data/Datatables/PowerUps/PowerUpsList_DT.PowerUpsList_DT"))
    (for _array_element _outrownames_2
      ;[0 0 0] Añade PowerUp con el nivel 0 a la tabla
      (bind _returnvalue (Utilities|GetDataTableRow "/Game/Blueprint/Data/Datatables/PowerUps/PowerUpsList_DT.PowerUpsList_DT" _array_element)
        (:then
          (if (not (.ReturnValue (Utilities|Map|Find (Variables|/Game/Blueprint/ManagersAndControllers/MainSaveGame.MainSaveGame_C|GetPowerUps (Variables|Default|GetSaveGameData)) (Utilities|Struct|BreakPowerUpsList_ST _returnvalue))))
            (Utilities|Map|Add (Variables|/Game/Blueprint/ManagersAndControllers/MainSaveGame.MainSaveGame_C|GetPowerUps (Variables|Default|GetSaveGameData)) (Utilities|Struct|BreakPowerUpsList_ST _returnvalue) 0)))))
    (SaveGame|SaveGame)))

(fn GetPowerUps
  (return (Variables|/Game/Blueprint/ManagersAndControllers/MainSaveGame.MainSaveGame_C|GetPowerUps (Variables|Default|GetSaveGameData))))

(fn AddPowerUp
  (params (Data :type Data%20Table%20Object%20Reference))
  (bind _savegamedata (Variables|Default|GetSaveGameData))
  (bind _powerups (Variables|/Game/Blueprint/ManagersAndControllers/MainSaveGame.MainSaveGame_C|GetPowerUps _savegamedata))
  (Utilities|Map|Add _powerups Data (+ (.Value (Utilities|Map|Find _powerups Data)) 1))
  (SaveGame|SaveGame)
  (return))

(fn RemovePowerUp
  (params (Data :type Data%20Table%20Object%20Reference))
  (bind _savegamedata (Variables|Default|GetSaveGameData))
  (bind _powerups (Variables|/Game/Blueprint/ManagersAndControllers/MainSaveGame.MainSaveGame_C|GetPowerUps _savegamedata))
  (Utilities|Map|Add _powerups Data (- (.Value (Utilities|Map|Find _powerups Data)) 1))
  (SaveGame|SaveGame)
  (return))

(fn CalcPowerUpStats
  (bind _powerupstats (Variables|PowerUp|GetPowerUpStats))
  (bind (_hpstructure _movespeedmultiplier _damagemultiplier _projectilespeedmultiplier _areamultiplier _projectilenumber _projectileduration _rateoffiremultiplier _luck _expmultiplier _moneymultiplier _pickarea _skips _discard _reroll _curse) (Utilities|Struct|BreakPlayerStructure _powerupstats))
  (bind _keys (Utilities|Map|Keys (Variables|/Game/Blueprint/ManagersAndControllers/MainSaveGame.MainSaveGame_C|GetPowerUps (Variables|Default|GetSaveGameData))))
  (for _array_element _keys
    (if (not (== (.Value (Utilities|Map|Find (Variables|/Game/Blueprint/ManagersAndControllers/MainSaveGame.MainSaveGame_C|GetPowerUps (Variables|Default|GetSaveGameData)) _array_element)) 0))
      (bind _returnvalue (Utilities|GetDataTableRow _array_element (Utilities|String|StringToName (Utilities|String|ToString(Integer) (.Value (Utilities|Map|Find (Variables|/Game/Blueprint/ManagersAndControllers/MainSaveGame.MainSaveGame_C|GetPowerUps (Variables|Default|GetSaveGameData)) _array_element)))))
        (:then
          (Utilities|Struct|SetmembersinPlayerStructure (Variables|PowerUp|GetPowerUpStats) (Utilities|Struct|MakeHp_Structure (+ (.hpmax (.HpStructure (Utilities|Struct|BreakPlayerStructure (.Data (Utilities|Struct|BreakPowerUps_ST _returnvalue))))) (.hpmax _hpstructure)) (+ (.currenthp (.HpStructure (Utilities|Struct|BreakPlayerStructure (.Data (Utilities|Struct|BreakPowerUps_ST _returnvalue))))) (.currenthp _hpstructure)) (+ (.armor (.HpStructure (Utilities|Struct|BreakPlayerStructure (.Data (Utilities|Struct|BreakPowerUps_ST _returnvalue))))) (.armor _hpstructure)) (+ (.recoveryhp (.HpStructure (Utilities|Struct|BreakPlayerStructure (.Data (Utilities|Struct|BreakPowerUps_ST _returnvalue))))) (.recoveryhp _hpstructure)) (+ (.lifes (.HpStructure (Utilities|Struct|BreakPlayerStructure (.Data (Utilities|Struct|BreakPowerUps_ST _returnvalue))))) (.lifes _hpstructure))) (+ (.MoveSpeedMultiplier (Utilities|Struct|BreakPlayerStructure (.Data (Utilities|Struct|BreakPowerUps_ST _returnvalue)))) _movespeedmultiplier) (+ (.DamageMultiplier (Utilities|Struct|BreakPlayerStructure (.Data (Utilities|Struct|BreakPowerUps_ST _returnvalue)))) _damagemultiplier) (+ (.ProjectileSpeedMultiplier (Utilities|Struct|BreakPlayerStructure (.Data (Utilities|Struct|BreakPowerUps_ST _returnvalue)))) _projectilespeedmultiplier) (+ (.AreaMultiplier (Utilities|Struct|BreakPlayerStructure (.Data (Utilities|Struct|BreakPowerUps_ST _returnvalue)))) _areamultiplier) (+ (.ProjectileNumber (Utilities|Struct|BreakPlayerStructure (.Data (Utilities|Struct|BreakPowerUps_ST _returnvalue)))) _projectilenumber) (+ (.ProjectileDuration (Utilities|Struct|BreakPlayerStructure (.Data (Utilities|Struct|BreakPowerUps_ST _returnvalue)))) _projectileduration) (+ (.RateOfFireMultiplier (Utilities|Struct|BreakPlayerStructure (.Data (Utilities|Struct|BreakPowerUps_ST _returnvalue)))) _rateoffiremultiplier) (+ (.Luck (Utilities|Struct|BreakPlayerStructure (.Data (Utilities|Struct|BreakPowerUps_ST _returnvalue)))) _luck) (+ (.ExpMultiplier (Utilities|Struct|BreakPlayerStructure (.Data (Utilities|Struct|BreakPowerUps_ST _returnvalue)))) _expmultiplier) (+ (.MoneyMultiplier (Utilities|Struct|BreakPlayerStructure (.Data (Utilities|Struct|BreakPowerUps_ST _returnvalue)))) _moneymultiplier) (+ (.PickArea (Utilities|Struct|BreakPlayerStructure (.Data (Utilities|Struct|BreakPowerUps_ST _returnvalue)))) _pickarea) (+ (.Skips (Utilities|Struct|BreakPlayerStructure (.Data (Utilities|Struct|BreakPowerUps_ST _returnvalue)))) _skips) (+ (.Discard (Utilities|Struct|BreakPlayerStructure (.Data (Utilities|Struct|BreakPowerUps_ST _returnvalue)))) _discard) (+ (.Reroll (Utilities|Struct|BreakPlayerStructure (.Data (Utilities|Struct|BreakPowerUps_ST _returnvalue)))) _reroll) (+ (.Curse (Utilities|Struct|BreakPlayerStructure (.Data (Utilities|Struct|BreakPowerUps_ST _returnvalue)))) _curse)))))))

(fn ApplyPowerUps
  (bind _powerupstats (Variables|PowerUp|GetPowerUpStats))
  (bind _characterselected (Variables|Default|GetCharacterSelected))
  (bind _characterstats (Utilities|Struct|BreakUI_CharacterStructure _characterselected))
  (bind (_hpstructure _movespeedmultiplier _damagemultiplier _projectilespeedmultiplier _areamultiplier _projectilenumber _projectileduration _rateoffiremultiplier _luck _expmultiplier _moneymultiplier _pickarea _skips _discard _reroll _curse) (Utilities|Struct|BreakPlayerStructure _powerupstats))
  (bind (_hpstructure_2 _movespeedmultiplier_2 _damagemultiplier_2 _projectilespeedmultiplier_2 _areamultiplier_2 _projectilenumber_2 _projectileduration_2 _rateoffiremultiplier_2 _luck_2 _expmultiplier_2 _moneymultiplier_2 _pickarea_2 _skips_2 _discard_2 _reroll_2 _curse_2) (Utilities|Struct|BreakPlayerStructure _characterstats))
  (Utilities|Struct|SetmembersinPlayerStructure (Utilities|Struct|BreakUI_CharacterStructure (Variables|Default|GetCharacterSelected)) (Utilities|Struct|MakeHp_Structure (+ (.hpmax _hpstructure_2) (.hpmax _hpstructure)) (+ (.currenthp _hpstructure_2) (.currenthp _hpstructure)) (+ (.armor _hpstructure_2) (.armor _hpstructure)) (+ (.recoveryhp _hpstructure_2) (.recoveryhp _hpstructure)) (+ (.lifes _hpstructure_2) (.lifes _hpstructure))) (+ _movespeedmultiplier_2 _movespeedmultiplier) (+ _damagemultiplier_2 _damagemultiplier) (+ _projectilespeedmultiplier_2 _projectilespeedmultiplier) (+ _areamultiplier_2 _areamultiplier) (+ _projectilenumber_2 _projectilenumber) (+ _projectileduration_2 _projectileduration) (+ _rateoffiremultiplier_2 _rateoffiremultiplier) (+ _luck_2 _luck) (+ _expmultiplier_2 _expmultiplier) (+ _moneymultiplier_2 _moneymultiplier) (+ _pickarea_2 _pickarea) (+ _skips_2 _skips) (+ _discard_2 _discard) (+ _reroll_2 _reroll) (+ _curse_2 _curse))
  (return))