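; StatsComponent is an actor component that holds a character's upgradeable stats and combat tallies, covering health, combat multipliers, pickups, luck, curse and reroll-style charges.
; Update adds an incoming stat struct field by field onto the stored one, so changes stack additively, then fires an update dispatcher.
; Separate functions count enemy deaths and accumulate damage dealt per weapon in a map.
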(event EventBeginPlay)

(event EventTick
  (params (DeltaSeconds :type Float%20%28single-precision%29)))

(fn Update
  (params (UpdateInfo :type Player%20Structure%20Structure))
  (Variables|Default|SetStructure (Utilities|Struct|MakePlayerStructure (Utilities|Struct|MakeHp_Structure (+ (.hpmax (.hpstructure UpdateInfo)) (.hpmax (.hpstructure (Variables|Default|GetStructure)))) (+ (.currenthp (.hpstructure UpdateInfo)) (.currenthp (.hpstructure (Variables|Default|GetStructure)))) (+ (.armor (.hpstructure UpdateInfo)) (.armor (.hpstructure (Variables|Default|GetStructure)))) (+ (.recoveryhp (.hpstructure UpdateInfo)) (.recoveryhp (.hpstructure (Variables|Default|GetStructure)))) (+ (.lifes (.hpstructure UpdateInfo)) (.lifes (.hpstructure (Variables|Default|GetStructure))))) (+ (.movespeedmultiplier UpdateInfo) (.movespeedmultiplier (Variables|Default|GetStructure))) (+ (.damagemultiplier UpdateInfo) (.damagemultiplier (Variables|Default|GetStructure))) (+ (.areamultiplier UpdateInfo) (.areamultiplier (Variables|Default|GetStructure))) (+ (.projectilespeedmultiplier UpdateInfo) (.projectilespeedmultiplier (Variables|Default|GetStructure))) (+ (.projectilenumber UpdateInfo) (.projectilenumber (Variables|Default|GetStructure))) (+ (.projectileduration UpdateInfo) (.projectileduration (Variables|Default|GetStructure))) (+ (.rateoffiremultiplier UpdateInfo) (.rateoffiremultiplier (Variables|Default|GetStructure))) (+ (.luck UpdateInfo) (.luck (Variables|Default|GetStructure))) (+ (.expmultiplier UpdateInfo) (.expmultiplier (Variables|Default|GetStructure))) (+ (.moneymultiplier UpdateInfo) (.moneymultiplier (Variables|Default|GetStructure))) (+ (.pickarea UpdateInfo) (.pickarea (Variables|Default|GetStructure))) (+ (.skips UpdateInfo) (.skips (Variables|Default|GetStructure))) (+ (.discard UpdateInfo) (.discard (Variables|Default|GetStructure))) (+ (.reroll UpdateInfo) (.reroll (Variables|Default|GetStructure))) (+ (.curse UpdateInfo) (.curse (Variables|Default|GetStructure)))))
  (Default|CallCallUptade)
  (return true))

(fn AddEnemyDeath
  (Math|Integer|IncrementInt (Variables|Default|GetEnemyDeaths)
    (:%20%20
      (return true))))

(fn AddDamageStat
  (params (DamageToAdd :type Float%20%28double-precision%29%20%28by%20ref%29) (Weapon :type Data%20Table%20Object%20Reference%20%28by%20ref%29))
  (Utilities|Map|Add (Variables|Default|GetWeaponStats) Weapon (+ (.Value (Utilities|Map|Find (Variables|Default|GetWeaponStats) Weapon)) DamageToAdd))
  (return true))