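; Player pawn for what appears to be a survivors-style game, moved by axis input through FloatingPawnMovement and yawed toward its velocity.
; After a short delay it wires stats, HP, weapon, item and spawner components together, equips default Knifes and creates the HUD.
; A per-tick sphere trace sized by PickArea triggers pickup magnets, whose drops feed scaled XP to LvlSystem.
; Damage routes through HpSystem, spawning floating text and showing end-game on death.
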(event Custom|StartPlayer
  (CallFunction|Initialite)
  ;[0 0 0 1 12] Arma por defecto, conector esto en el futuro con el arma del jugador elegido
  (Default|AddWeapon (Variables|Default|GetWeaponSystem) "/Game/Blueprint/Weapon/DataTables/Knifes.Knifes")
  ;[1 1 1] Creamos interfaz
  (bind _returnvalue (UserInterface|CreateWidget "/Game/Blueprint/Interfaz/HUDWidget.HUDWidget_C" 0 (Variables|Default|GetWeaponSystem) (Variables|Default|GetItemSystem) (Variables|Default|GetStatsComponent) (Variables|Default|GetHp_System) (Variables|Default|GetLvlSystem)))
  (bind _output_get (Variables|Default|SetHudReference _returnvalue))
  (UserInterface|Viewport|AddtoViewport _output_get 0)
  (Variables|/Game/Blueprint/LvlSystem/LvlSystem.LvlSystem_C|SetHudRefence (Variables|Default|GetLvlSystem) (Variables|Default|GetHudReference))
  ;[0 0 0 1 12] Vinculamos al player con el evento de update stats
  (EventDispatchers|BindEventtoCallUptade (Variables|Default|GetStatsComponent) (EventDispatchers|CreateEvent :!event CheckUpdate))
  ;[0 0 0 1 10] Comprobamos si hay recovery
  (Default|CheckRecovery (Variables|Default|GetHp_System))
  (Variables|/Game/Blueprint/StatComponent/StatsComponent.StatsComponent_C|SetStartDeltaTime (Variables|Default|GetStatsComponent) (Utilities|Time|GetGameTimeinSeconds)))

(event EventTick
  (params (DeltaSeconds :type Float%20%28single-precision%29))
  (bind _returnvalue (Transformation|GetVelocity))
  (CallFunction|InteractwithObjets)
  (if (Utilities|Operators|NotEqual(!=) :A _returnvalue :ErrorTolerance 4.0)
    (Transformation|AddActorLocalRotation (Math|Rotator|MakeRotator 0.0 0.0 (Class|KismetAnimationLibrary|CalculateDirection _returnvalue (Transformation|GetActorRotation))) false false)))

(event EventDropInteract
  (params (Xp? :type Float%20%28double-precision%29))
  (bind _statscomponent (Variables|Default|GetStatsComponent))
  (bind _structure (Variables|/Game/Blueprint/StatComponent/StatsComponent.StatsComponent_C|GetStructure _statscomponent))
  (bind _expmultiplier (Utilities|Struct|BreakPlayerStructure _structure))
  ;[1 1 1] Añadimos XP
  (Default|AddXP (Variables|Default|GetLvlSystem) (* Xp? (Math|Float|SelectFloat 1.0 _expmultiplier (< _expmultiplier 1.0)))))

(event EventBeginPlay
  (Utilities|Time|SetTimerbyEvent (delegate Custom|StartPlayer) 0.5))

(event Input|AxisEvents|InputAxisMoveForward
  (params (AxisValue :type Float%20%28single-precision%29))
  ;[1 1 1] Movimiento del Personaje
  (Class|PawnMovementComponent|AddInputVector (Variables|Default|GetFloatingPawnMovement) (Math|Vector|MakeVector AxisValue 0.0 0.0) false))

(event Input|AxisEvents|InputAxisMoveLeft
  (params (AxisValue :type Float%20%28single-precision%29))
  ;[1 1 1] Movimiento del Personaje
  (Class|PawnMovementComponent|AddInputVector (Variables|Default|GetFloatingPawnMovement) (Math|Vector|MakeVector 0.0 AxisValue 0.0) false))

(event Input|KeyboardEvents|J
  (params (Key :type Key%20Structure :default "None"))
  ;[1 1 1] Debug
  (:Pressed
    (bind _returnvalue (UserInterface|CreateWidget "/Game/Blueprint/Interfaz/MainMenu/UI_MainMenu.UI_MainMenu_C"))
    (UserInterface|Viewport|AddtoViewport _returnvalue 0)
    (Game|SetGamePaused true)
    (Variables|/Script/Engine.PlayerController|SetbShowMouseCursor (Game|GetPlayerController 0) true)))

(event Input|KeyboardEvents|L
  (params (Key :type Key%20Structure :default "None"))
  ;[1 1 1] Debug
  (:Pressed
    (Default|LevelUp (Variables|Default|GetHudReference))))

(fn ConstructionScript)

(fn InteractwithObjets
  (bind _returnvalue (Transformation|GetActorLocation))
  ;[1 1 1] Detectamos los items para agregarlos, de momento solo la experiencia
  (bind (_outhit _returnvalue_2) (Collision|SphereTraceByChannel _returnvalue _returnvalue (.PickArea (Utilities|Struct|BreakPlayerStructure (Variables|/Game/Blueprint/StatComponent/StatsComponent.StatsComponent_C|GetStructure (Variables|Default|GetStatsComponent)))) "TraceTypeQuery3" false 0 "None"))
  (if _returnvalue_2
    (if (Utilities|DoesObjectImplementInterface (.HitActor (Collision|BreakHitResult _outhit)) "/Game/Blueprint/Vampire_Interaction.Vampire_Interaction_C")
      (Class|VampireInteraction|MagnetMode(Message) (.HitActor (Collision|BreakHitResult _outhit)) self))))

(fn CheckUpdate
  (bind _floatingpawnmovement (Variables|Default|GetFloatingPawnMovement))
  (Variables|/Script/Engine.FloatingPawnMovement|SetMaxSpeed _floatingpawnmovement (+ (Variables|/Script/Engine.FloatingPawnMovement|GetMaxSpeed _floatingpawnmovement) (.MoveSpeedMultiplier (Utilities|Struct|BreakPlayerStructure (Variables|/Game/Blueprint/StatComponent/StatsComponent.StatsComponent_C|GetStructure (Variables|Default|GetStatsComponent)))))))

(fn Loteria
  (LocalVariables|SetControlador 1)
  (LocalVariables|SetTotal 1)
  (for _array_element (Variables|Default|GetLoteriaProbs)
    (LocalVariables|SetTotal (+ (LocalVariables|GetTotal) _array_element)))
  (LocalVariables|SetGanador (Math|Random|RandomIntegerinRange (LocalVariables|GetControlador) (LocalVariables|GetTotal)))
  (bind (_array_element_2 _array_index) (Utilities|Array|ForEachLoopwithBreak (Variables|Default|GetLoteriaProbs) :!label _label)
    (:LoopBody
      (if (>= (+ (LocalVariables|GetControlador) _array_element_2) (LocalVariables|GetGanador))
        (LocalVariables|SetIndex _array_index)
        (goto _label Break)
        (else
          (LocalVariables|SetControlador (+ (LocalVariables|GetControlador) _array_element_2)))))
    (:Completed
      (Development|PrintString (Utilities|String|Append "Ganador!  - " (Utilities|String|ToString(Integer) (LocalVariables|GetIndex)) "- Con el numero - " (Utilities|String|ToString(Integer) (LocalVariables|GetGanador))) true true "(R=0.046794,G=1.000000,B=0.000000,A=1.000000)"))))

(fn Initialite
  (bind _weaponsystem (Variables|Default|GetWeaponSystem))
  (Variables|/Game/Blueprint/HpSystem/Hp_System.Hp_System_C|SetStatsComponent (Variables|Default|GetHp_System) (Variables|Default|GetStatsComponent))
  (Variables|/Game/Blueprint/ItemSystem/ItemSystem.ItemSystem_C|SetStatsComponent (Variables|Default|GetItemSystem) (Variables|Default|GetStatsComponent))
  (Variables|/Game/Blueprint/Weapon/WeaponSystem.WeaponSystem_C|SetStatsComponent _weaponsystem (Variables|Default|GetStatsComponent))
  (Variables|/Game/Blueprint/Weapon/WeaponSystem.WeaponSystem_C|SetPlayerReference _weaponsystem self)
  (Variables|/Game/Blueprint/Spawner/SpawnerComponent.SpawnerComponent_C|SetPlayerReference (Variables|Default|GetSpawnerComponent) self)
  (return))

(fn DamageInterface
  (params (Damage :type Float%20%28double-precision%29)))

(fn DamagetoPlayer
  (params (DamageToPlayer :type Float%20%28double-precision%29))
  (bind _returnvalue (Transformation|GetActorLocation))
  (bind (_dead_ _damagedeal) (Default|ApplyDamage (Variables|Default|GetHp_System) DamageToPlayer))
  (Game|SpawnActorfromClass "/Game/Blueprint/Interfaz/Bp_FloatingText.Bp_FloatingText_C" (Math|Transform|MakeTransform (Math|Vector|MakeVector (.x _returnvalue) (.y _returnvalue) (+ (.z _returnvalue) 8e+01)) "0, 0, 0" "1.000000,1.000000,1.000000") "AlwaysSpawn" 0 _damagedeal (Math|Color|MakeColor 255 0 0) 0)
  (if _dead_
    (Default|EndGameScreen (Variables|Default|GetHudReference)))
  (return false))

(fn MagnetMode
  (params (PlayerReference :type Actor%20Object%20Reference)))