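; Base unit for a tile-based tactics game that moves between terrain tiles and attacks enemy units.
; Sphere overlaps find the origin tile and reachable tiles; InteractWithTile moves onto a free tile or damages an opposing occupant and snaps back, then advances the turn through TacticsGameInstance.
; Tick interpolates movement until a timer expires, then snaps, refreshes range and re-enables grabbing.
; At zero HP the unit leaves the bag, is destroyed and triggers a win check.
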(event Custom|GetCurrentSocketLocation
  (bind _outactors (Collision|SphereOverlapActors (Transformation|GetActorLocation) 2e+01 (Utilities|Array|MakeArray "ObjectTypeQuery7") "/Game/Blueprint/Bp_Terrain.Bp_Terrain_C"))
  (for _array_element _outactors
    (bind _output_get (Variables|Default|SetOriginTile _array_element))
    (Development|PrintString (Utilities|GetDisplayName _output_get))))

(event EventBeginPlay
  (Rendering|Material|SetMaterial (Variables|Default|GetStaticMesh) 0 (Variables|Default|GetMaterial_Base))
  (CallFunction|TerrainatRange)
  (Variables|Default|SetCanbeGrab? true))

(event EventTick
  (params (DeltaSeconds :type Float%20%28single-precision%29))
  (if (Variables|MoveController|GetMove?)
    (CallFunction|Moveto)))

(fn ConstructionScript
  (Variables|Default|SetCanbeGrab? true))

(fn ApplyDamage
  (params (Damage :type Integer))
  (bind _output_get (Variables|Gameplay|SetHp (- (Variables|Gameplay|GetHp) Damage)))
  (Development|PrintString (Utilities|String|ToString(Integer) _output_get) true true "(R=0.677732,G=1.000000,B=0.000000,A=1.000000)")
  (if (<= _output_get 0)
    (Development|PrintString "Muerto")
    (bind _astactics_game_instance (Utilities|Casting|CastToTacticsGameInstance (Game|GetGameInstance)))
    (Default|RemoveChipfromBag _astactics_game_instance self)
    (Actor|DestroyActor)
    (Default|CheckWinCondition _astactics_game_instance)
    (else
      (Development|PrintString "Daño Aplicado"))))

(fn InteractwithTile
  (params (TargetTile :type Bp%20Terrain%20Object%20Reference) (NoTile :type Boolean))
  (if NoTile
    (CallFunction|ResetPosition)
    (elif (== TargetTile (Variables|Default|GetOriginTile))
      (CallFunction|ResetPosition)
      (else
        ;[1 1 1] Tile local Var
        (bind _output_get (LocalVariables|SetTile TargetTile))
        (if (== (Utilities|Array|FindItem (Variables|GridController|GetTilesAtRange) _output_get) -1)
          (CallFunction|ResetPosition)
          (else
            ;[1 1 1] Occupied?
            (if (Variables|/Game/Blueprint/Bp_Terrain.Bp_Terrain_C|GetEstaOcupada? _output_get)
              ;[1 1 1] Ocuppied, attack and reset move
              (bind _asbp_master_unit (Utilities|Casting|CastToBp_MasterUnit (Variables|/Game/Blueprint/Bp_Terrain.Bp_Terrain_C|GetQuienMeocupa (LocalVariables|GetTile))))
              (if (!= (Variables|Bp_MasterUnit_C|GetTeam _asbp_master_unit) (Variables|Gameplay|GetTeam))
                (CallFunction|ApplyDamage _asbp_master_unit (Variables|Gameplay|GetDamage)))
              (CallFunction|ResetPosition)
              ;[0.9768 0 1] GameInstance
              (bind _astactics_game_instance (Utilities|Casting|CastToTacticsGameInstance (Game|GetGameInstance)))
              (Default|NextTurnEvent _astactics_game_instance)
              (else
                ;[1 1 1] Not occupied, move
                (Variables|MoveController|SetTime? (Utilities|Time|GetGameTimeinSeconds))
                (Variables|MoveController|SetMoveTo (Transformation|GetSocketLocation (Variables|/Script/Engine.Actor|GetRootComponent (LocalVariables|GetTile)) "Centro"))
                (Variables|MoveController|SetMove? true)
                (Actor|Tick|SetActorTickEnabled true)
                ;[0.9768 0 1] GameInstance
                (bind _astactics_game_instance_2 (Utilities|Casting|CastToTacticsGameInstance (Game|GetGameInstance)))
                (Default|NextTurnEvent _astactics_game_instance_2)))))))))

(fn ResetPosition
  (Variables|MoveController|SetTime? (Utilities|Time|GetGameTimeinSeconds))
  (Variables|MoveController|SetMove? true)
  (Variables|MoveController|SetMoveTo (Transformation|GetActorLocation (Variables|Default|GetOriginTile)))
  (Actor|Tick|SetActorTickEnabled true))

(fn Moveto
  (bind _feebackgrabtime (Variables|MoveController|GetFeebackGrabTime))
  (if (>= (Utilities|Time|GetGameTimeinSeconds) (+ (Variables|MoveController|GetTime?) (Variables|MoveController|GetFeebackGrabTime)))
    (Transformation|SetActorLocation (Variables|MoveController|GetMoveTo) false false)
    (Variables|MoveController|SetMove? false)
    (Actor|Tick|SetActorTickEnabled false)
    (CallFunction|TerrainatRange)
    (Variables|Default|SetCanbeGrab? true)
    (Rendering|Material|SetMaterial (Variables|Default|GetStaticMesh) 0 (Variables|Default|GetMaterial_Base))
    (else
      (Transformation|SetActorLocation (Math|Interpolation|VInterpTo (Transformation|GetActorLocation) (Variables|MoveController|GetMoveTo) _feebackgrabtime _feebackgrabtime) false false))))

(fn TerrainatRange
  (bind _outactors (Collision|SphereOverlapActors (Transformation|GetActorLocation) 1e+02 (Utilities|Array|MakeArray "ObjectTypeQuery7") "/Game/Blueprint/Bp_Terrain.Bp_Terrain_C"))
  (Variables|GridController|SetTilesAtRange _outactors))